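; Player-controlled Paper2D character with eight-way movement and depth sorting on a layered tilemap, apparently isometric.
; BeginPlay scans the first PaperTileActor, caching tile positions, diagonal layer indices (X+Y), edge-tile bounds and the depth range.
; Each tick pins the flipbook to the capsule, mapping its half-tile-snapped Y to a Z between cosmetic layers.
; Axis input drives movement and the last direction, which selects run or idle flipbook and capsule yaw.
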(event `self.ReceiveBeginPlay`
  (bind _layerzvaluemap (`self.LayerZValueMap`))
  (bind _returnvalue (`KismetMathLibrary.Abs` (/ (`self.TileWidth`) 2.0)))
  (bind _returnvalue_2 (`KismetMathLibrary.Abs` (/ (`self.TileHeight`) 2.0)))
  (bind _outactors (`GameplayStatics.GetAllActorsOfClass` "/Game/PaperTileActor.PaperTileActor_C"))
  (bind _output_get (set `self.CurTilemap` (`|GetArrayItem` _outactors)))
  (bind _rendercomponent (`PaperTileMapActor.RenderComponent` _output_get))
  (bind (_mapwidth _mapheight _numlayers) (`PaperTileMapComponent.GetMapSize` _rendercomponent))
  (set `self.NumCosmeticLayers` _numlayers)
  (`KismetSystemLibrary.PrintString` (`KismetStringLibrary.Concat_StrStr` (`KismetStringLibrary.Conv_IntToString` _mapwidth) ":" (`KismetStringLibrary.Conv_IntToString` _mapheight)) true true (struct :`G` 0.66 :`B` 1.0 :`A` 1.0) 20.0)
  (`BlueprintMapLibrary.Map_Clear` (`self.TileCoordsAndSimLayer`))
  (`BlueprintMapLibrary.Map_Clear` (`self.TileCoordsAndVector`))
  (for _index (range _mapwidth)
    (bind _returnvalue_3 (- _mapheight 1))
    (for _index_2 (range (+ _returnvalue_3 1))
      (bind _output_get_2 (set `self.SimulatedLayer` (+ _index _index_2)))
      (bind _returnvalue_4 (`KismetMathLibrary.Conv_IntToDouble` _index))
      (bind _returnvalue_5 (`KismetMathLibrary.Conv_IntToDouble` _index_2))
      (`BlueprintMapLibrary.Map_Add` (`self.TileCoordsAndSimLayer`) (`KismetMathLibrary.MakeVector2D` _returnvalue_4 _returnvalue_5) _output_get_2)
      (bind _returnvalue_6 (`PaperTileMapComponent.GetTileCenterPosition` _rendercomponent _index _index_2 0 true))
      (`BlueprintMapLibrary.Map_Add` (`self.TileCoordsAndVector`) (`KismetMathLibrary.MakeVector2D` _returnvalue_4 _returnvalue_5) _returnvalue_6)
      (if (or (== _index 0) (== _index_2 _returnvalue_3))
        (bind _x (.x _returnvalue_6))
        (bind _y (.y _returnvalue_6))
        (`BlueprintMapLibrary.Map_Add` (`self.LayerZValueMap`) _output_get_2 (- _y 0.0))
        (bind _output_get_3 (set `self.TileBounds` (make `/Game/TileCoordBounds` (+ _y _returnvalue_2) (- _y _returnvalue_2) (+ _x _returnvalue) (- _x _returnvalue))))
        (`BlueprintMapLibrary.Map_Add` (`self.TileCoordsAndBounds`) _output_get_3 (`KismetMathLibrary.MakeVector2D` _returnvalue_4 _returnvalue_5))
        (bind _values (`BlueprintMapLibrary.Map_Values` _layerzvaluemap))
        (set `self.MinMaxZOfTilemapForDepth` (`KismetMathLibrary.MakeVector2D` (`|GetArrayItem` _values) (`|GetArrayItem` _values (- (`BlueprintMapLibrary.Map_Length` _layerzvaluemap) 1))))))))

(event `self.ReceiveTick`
  (params (DeltaSeconds :type "Float (single-precision)"))
  (bind _sprite (`self.Sprite`))
  (bind (_minmaxzoftilemapfordepth_x _minmaxzoftilemapfordepth_y) (`KismetMathLibrary.BreakVector2D` (`self.MinMaxZOfTilemapForDepth`)))
  (bind (_returnvalue_x _returnvalue_y) (`KismetMathLibrary.BreakVector` (`SceneComponent.K2_GetComponentLocation` (`self.CapsuleComponent`))))
  (bind _returnvalue (/ (`self.TileHeight`) 2.0))
  (`SceneComponent.K2_SetWorldLocation` _sprite (`KismetMathLibrary.MakeVector` _returnvalue_x (- _returnvalue_y (`self.SpriteOffset`)) (+ (`KismetMathLibrary.MapRangeClamped` (`KismetMathLibrary.Conv_IntToDouble` (* (`.ReturnValue` (`KismetMathLibrary.FMod` (+ _returnvalue_y 0.0) _returnvalue)) (`KismetMathLibrary.FTrunc` _returnvalue))) _minmaxzoftilemapfordepth_x _minmaxzoftilemapfordepth_y (* (* (- (`self.NumCosmeticLayers`) 2) (`self.LayerSeparation`)) -1.0) 0.0) 0.0)) false false)
  (`SceneComponent.K2_SetWorldRotation` _sprite (struct :`Roll` -90.0) false false)
  (`self.SetFlipBookOnSprite`))

(event `InputAxis|UpDown`
  (params (AxisValue :type "Float (single-precision)"))
  (bind _gamepadsensitivity (`self.GamepadSensitivity`))
  (if (> AxisValue _gamepadsensitivity)
    (set `self.UpDownValueToPass` -1.0)
    (if (== (`self.RightLeftValueToPass`) 0.0) :!label _label
      (set `self.AddMovementY` (0.0 0.5 0.0))
      (else
        (set `self.AddMovementY` (0.0 0.5 0.0))))
    (elif (< AxisValue (* _gamepadsensitivity -1.0))
      (set `self.UpDownValueToPass` 1.0)
      (goto _label)
      (else
        (set `self.UpDownValueToPass` 0.0))))
  (`self.AddMovementInput` (`self.AddMovementY`) (`self.UpDownValueToPass`)))

(event `InputAxis|RightLeft`
  (params (AxisValue :type "Float (single-precision)"))
  (bind _gamepadsensitivity (`self.GamepadSensitivity`))
  (if (> AxisValue _gamepadsensitivity)
    (set `self.RightLeftValueToPass` 1.0)
    (if (== (`self.UpDownValueToPass`) 0.0) :!label _label_2
      (set `self.AddMovementX` (1.0 0.0 0.0))
      (else
        (set `self.AddMovementX` (1.0 0.0 0.0))))
    (elif (< AxisValue (* _gamepadsensitivity -1.0))
      (set `self.RightLeftValueToPass` -1.0)
      (goto _label_2)
      (else
        (set `self.RightLeftValueToPass` 0.0))))
  (`self.AddMovementInput` (`self.AddMovementX`) (`self.RightLeftValueToPass`)))

(fn `SetFlipBookOnSprite`
  (bind _rightleftvaluetopass (`self.RightLeftValueToPass`))
  (bind _lastmovedirection (`self.LastMoveDirection`))
  (bind _returnvalue (> _rightleftvaluetopass 0.0))
  (bind _returnvalue_2 (< _rightleftvaluetopass 0.0))
  (bind _returnvalue_3 (== _rightleftvaluetopass 0.0))
  (bind _returnvalue_4 (* (`self.UpDownValueToPass`) -1.0))
  (bind _returnvalue_5 (< _returnvalue_4 0.0))
  (bind _returnvalue_6 (> _returnvalue_4 0.0))
  (if (or (!= (`self.UpDownValueToPass`) 0.0) (!= (`self.RightLeftValueToPass`) 0.0))
    (set `self.LastMoveDirection` (select `bool` (and _returnvalue_6 _returnvalue) :`false` (select `bool` (and _returnvalue_6 _returnvalue_3) :`false` (select `bool` (and _returnvalue_6 _returnvalue_2) :`false` (select `bool` (and (== _returnvalue_4 0.0) _returnvalue_2) :`false` (select `bool` (and _returnvalue_5 _returnvalue_2) :`false` (select `bool` (and _returnvalue_5 _returnvalue_3) :`false` (select `bool` (and _returnvalue_5 _returnvalue) :`false` "NewEnumerator1" :`true` "NewEnumerator2" :!type "/Game/Character/EMoveDirection Enum") :`true` "NewEnumerator3") :`true` "NewEnumerator4") :`true` "NewEnumerator5") :`true` "NewEnumerator6") :`true` "NewEnumerator7") :`true` "NewEnumerator0")))
  (`PaperFlipbookComponent.SetFlipbook` (`self.Sprite`) (select `bool` (> (`KismetMathLibrary.VSize` (`self.GetVelocity`)) 0.0) :`false` (select `/Game/Character/EMoveDirection` _lastmovedirection :`NewEnumerator0` "/Game/Character/FlipBooks/Idle_N.Idle_N" :`NewEnumerator1` "/Game/Character/FlipBooks/Idle_NE.Idle_NE" :`NewEnumerator2` "/Game/Character/FlipBooks/Idle_E.Idle_E" :`NewEnumerator3` "/Game/Character/FlipBooks/Idle_SE.Idle_SE" :`NewEnumerator4` "/Game/Character/FlipBooks/Idle_S.Idle_S" :`NewEnumerator5` "/Game/Character/FlipBooks/Idle_SW.Idle_SW" :`NewEnumerator6` "/Game/Character/FlipBooks/Idle_W.Idle_W" :`NewEnumerator7` "/Game/Character/FlipBooks/Idle_NW.Idle_NW" :!type "PaperFlipbook Object Reference") :`true` (select `/Game/Character/EMoveDirection` _lastmovedirection :`NewEnumerator0` "/Game/Character/FlipBooks/Run_N.Run_N" :`NewEnumerator1` "/Game/Character/FlipBooks/Run_NE.Run_NE" :`NewEnumerator2` "/Game/Character/FlipBooks/Run_E.Run_E" :`NewEnumerator3` "/Game/Character/FlipBooks/Run_SE.Run_SE" :`NewEnumerator4` "/Game/Character/FlipBooks/Run_S.Run_S" :`NewEnumerator5` "/Game/Character/FlipBooks/Run_SW.Run_SW" :`NewEnumerator6` "/Game/Character/FlipBooks/Run_W.Run_W" :`NewEnumerator7` "/Game/Character/FlipBooks/Run_NW.Run_NW" :!type "PaperFlipbook Object Reference")))
  (`SceneComponent.K2_SetWorldRotation` (`self.CapsuleComponent`) (select `/Game/Character/EMoveDirection` (`self.LastMoveDirection`) :`NewEnumerator0` (struct :`Yaw` 335.0) :`NewEnumerator1` (struct) :`NewEnumerator2` (struct :`Yaw` 30.0) :`NewEnumerator3` (struct :`Yaw` 90.0) :`NewEnumerator4` (struct :`Yaw` 150.0) :`NewEnumerator5` (struct :`Yaw` 180.0) :`NewEnumerator6` (struct :`Yaw` 210.0) :`NewEnumerator7` (struct :`Yaw` 270.0) :!type "Rotator Structure") false false))

(fn `UserConstructionScript`
  (`SceneComponent.K2_SetWorldLocation` (`self.Sprite`) (`SceneComponent.K2_GetComponentLocation` (`self.CapsuleComponent`)) false false))