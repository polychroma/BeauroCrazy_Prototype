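; Behavior tree task that picks the next room for a BP_PaperNPC to patrol.
; It loops over the NPC's accessible rooms, skips searched ones and finds the closest by distance to each room's target point.
; That room joins SearchedRooms and goes to the RoomToSearch blackboard key before the task succeeds.
; Once searched and accessible counts match, it never calls FinishExecute, and SearchedRooms is never cleared here.
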(event `self.ReceiveExecuteAI`
  (params (OwnerController :type "AIController Object Reference") (ControlledPawn :type "Pawn Object Reference"))
  (set `self.LoopFirstPass` true)
  (set `self.ClosestRoom` null)
  (set `self.ClosestRoomDistance` 0.0)
  (bind _asbp_paper_npc (cast `/Game/Characters/BP_PaperNPC` ControlledPawn))
  (bind _output_get (set `self.AccessibleRooms` (`/Game/Characters/BP_PaperCharacterParent.AccessibleRooms` _asbp_paper_npc)))
  (for _array_element _output_get
    (if (`KismetArrayLibrary.Array_Contains` (`self.SearchedRooms`) _array_element)
      _
      (elif (`self.LoopFirstPass`)
        (set `self.ClosestRoom` _array_element)
        (set `self.LoopFirstPass` false)
        (bind _returnvalue (`KismetMathLibrary.VSize` (- (`Actor.K2_GetActorLocation` (`/Game/Environment/Rooms/BP_Room.AssociatedTargetPoint` _array_element)) (`Actor.K2_GetActorLocation` ControlledPawn))))
        (set `self.ClosestRoomDistance` _returnvalue)
        (elif (< _returnvalue (`self.ClosestRoomDistance`))
          (set `self.ClosestRoomDistance` _returnvalue)
          (set `self.ClosestRoom` _array_element)))))
  (if (not (== (`KismetArrayLibrary.Array_Length` (`self.SearchedRooms`)) (`KismetArrayLibrary.Array_Length` (`self.AccessibleRooms`))))
    (`KismetArrayLibrary.Array_AddUnique` (`self.SearchedRooms`) (`self.ClosestRoom`))
    (`BTFunctionLibrary.SetBlackboardValueAsObject` (`self.RoomToSearch`) (`self.ClosestRoom`))
    (`self.FinishExecute` true)))