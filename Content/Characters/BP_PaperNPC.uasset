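; Paper2D NPC character for a tilemap world, with axis-input movement, eight-direction idle/run flipbooks and dialogue participation.
; BeginPlay caches tile centers and depth range from the first tilemap; Tick picks the flipbook, rotates the capsule and maps its row-snapped Y to sprite Z for depth sorting.
; Helpers manage a per-NPC dialogue widget with name override and timeout hiding or removal.
; Most dialogue participant functions are stubs, and the radius overlap does nothing.
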(event `self.ReceiveBeginPlay`
  (bind _outactors (`GameplayStatics.GetAllActorsOfClass` "/Game/IsometricTiles/TileMaps/TileMapActor.TileMapActor_C"))
  (bind _output_get (set `self.CurTilemap` (`|GetArrayItem` _outactors)))
  (`self.GetLayerInformationForCharSprites` (`PaperTileMapActor.RenderComponent` _output_get)))

(event `self.ReceiveTick`
  (params (DeltaSeconds :type "Float (single-precision)"))
  (`self.Set Sprite Depth Layer`)
  (`self.SetFlipBookOnSprite`)
  (`self.DLGTimeoutLogic`))

(event `InputAxis|UpDown`
  (params (AxisValue :type "Float (single-precision)"))
  (bind _gamepadsensitivity (`self.GamepadSensitivity`))
  ;[1 1 1] Movement
  (if (> AxisValue _gamepadsensitivity)
    (set `self.UpDownValueToPass` -1.0)
    (if (== (`self.RightLeftValueToPass`) 0.0) :!label _label
      (set `self.AddMovementY` (0.0 0.5 0.0))
      (else
        (set `self.AddMovementY` (0.0 0.5 0.0))))
    (elif (< AxisValue (* _gamepadsensitivity -1.0))
      (set `self.UpDownValueToPass` 1.0)
      (goto _label)
      (else
        (set `self.UpDownValueToPass` 0.0))))
  (`self.AddMovementInput` (`self.AddMovementY`) (`self.UpDownValueToPass`)))

(event `InputAxis|RightLeft`
  (params (AxisValue :type "Float (single-precision)"))
  (bind _gamepadsensitivity (`self.GamepadSensitivity`))
  ;[1 1 1] Movement
  (if (> AxisValue _gamepadsensitivity)
    (set `self.RightLeftValueToPass` 1.0)
    (if (== (`self.UpDownValueToPass`) 0.0) :!label _label_2
      (set `self.AddMovementX` (1.0 0.0 0.0))
      (else
        (set `self.AddMovementX` (1.0 0.0 0.0))))
    (elif (< AxisValue (* _gamepadsensitivity -1.0))
      (set `self.RightLeftValueToPass` -1.0)
      (goto _label_2)
      (else
        (set `self.RightLeftValueToPass` 0.0))))
  (`self.AddMovementInput` (`self.AddMovementX`) (`self.RightLeftValueToPass`)))

(event `self.DialogueRadius.OnComponentBeginOverlap`
  (params (OverlappedComponent :type "PrimitiveComponent Object Reference") (OtherActor :type "Actor Object Reference") (OtherComp :type "PrimitiveComponent Object Reference") (OtherBodyIndex :type Integer) (bFromSweep :type Boolean) (SweepResult :type "HitResult Structure (by ref)"))
  (if (== (`GameplayStatics.GetObjectClass` OtherActor) "/Game/Characters/BP_PaperPC.BP_PaperPC_C")
    (bind _asbp_paper_pc (cast `/Game/Characters/BP_PaperPC` OtherActor))
    (if (== OtherComp (`/Game/Characters/BP_PaperPC.DialogueRadius` _asbp_paper_pc))
      _)))

(event `DLGCallToPossessCharacter`
  ;[1 1 1] TODO: If going a different route than StartDay, will need to figure out a function (outside of this class) that can be called from dialogues when possessing a character. loooks like this
  (set `self.DialogueWithPlayer` false))

(fn `CheckCondition`
  (params (Context :type "DlgContext Object Reference") (ConditionName :type Name))
  (returns (ReturnValue :type Boolean))
  (return false))

(fn `DLGTimeoutLogic`
  (bind _dlgwidget (`self.DLGWidget`))
  (bind _dlgwidget_2 (`self.DLGWidget`))
  (if (`self.DLGVis`)
    (set `self.DialogueTimer` (`KismetSystemLibrary.GetGameTimeInSeconds`))
    (else
      (if (> (- (`KismetSystemLibrary.GetGameTimeInSeconds`) (`self.DialogueTimer`)) (`self.DialogueTimeout`))
        (if (`self.DialogueWithPlayer`)
          (`/Engine/EditorBlueprintResources/StandardMacros.IsValid` _dlgwidget_2 :!label _label
            (:`Is Valid`
              (`Widget.SetVisibility` _dlgwidget_2 "Hidden"))
            (:`Is Not Valid`
              _))
          (elif (`self.DialogueWithNPC`)
            (goto _label)
            (else
              (`/Engine/EditorBlueprintResources/StandardMacros.IsValid` _dlgwidget
                (:`Is Valid`
                  (`Widget.RemoveFromParent` _dlgwidget)
                  (set `self.DLGWidget` null))
                (:`Is Not Valid`
                  _))))))
      (return))))

(fn `GetBoolValue`
  (params (ValueName :type Name))
  (returns (ReturnValue :type Boolean))
  (return false))

(fn `GetFloatValue`
  (params (ValueName :type Name))
  (returns (ReturnValue :type "Float (double-precision)"))
  (return 0.0))

(fn `GetIntValue`
  (params (ValueName :type Name))
  (returns (ReturnValue :type Integer))
  (return 0))

(fn `GetLayerInformationForCharSprites`
  (params (PaperTileMap :type "PaperTileMapComponent Object Reference"))
  (bind _layerzvaluemap (`self.LayerZValueMap`))
  (bind _returnvalue (`KismetMathLibrary.Abs` (/ (`self.TileWidth`) 2.0)))
  (bind _returnvalue_2 (`KismetMathLibrary.Abs` (/ (`self.TileHeight`) 2.0)))
  (bind (_mapwidth _mapheight _numlayers) (`PaperTileMapComponent.GetMapSize` PaperTileMap))
  (set `self.NumCosmeticLayers` _numlayers)
  (`KismetSystemLibrary.PrintString` (`KismetStringLibrary.Concat_StrStr` (`KismetStringLibrary.Conv_IntToString` _mapwidth) ":" (`KismetStringLibrary.Conv_IntToString` _mapheight)) true true (struct :`G` 0.66 :`B` 1.0 :`A` 1.0) 20.0)
  (`BlueprintMapLibrary.Map_Clear` (`self.TileCoordsAndSimLayer`))
  (`BlueprintMapLibrary.Map_Clear` (`self.TileCoordsAndVector`))
  ;[1 1 1] Loop for each X by Y in the tile map
  (for _index (range _mapwidth)
    (bind _returnvalue_3 (- _mapheight 1))
    (for _index_2 (range (+ _returnvalue_3 1))
      (bind _output_get (set `self.SimulatedLayer` (+ _index _index_2)))
      (bind _returnvalue_4 (`KismetMathLibrary.Conv_IntToDouble` _index))
      (bind _returnvalue_5 (`KismetMathLibrary.Conv_IntToDouble` _index_2))
      ;[1 1 1] Intermediate step of getting layer by tile coords, also gives center location for each tile coord
      (`BlueprintMapLibrary.Map_Add` (`self.TileCoordsAndSimLayer`) (`KismetMathLibrary.MakeVector2D` _returnvalue_4 _returnvalue_5) _output_get)
      (bind _returnvalue_6 (`PaperTileMapComponent.GetTileCenterPosition` PaperTileMap _index _index_2 0 true))
      (`BlueprintMapLibrary.Map_Add` (`self.TileCoordsAndVector`) (`KismetMathLibrary.MakeVector2D` _returnvalue_4 _returnvalue_5) _returnvalue_6)
      ;[1 1 1] Get depth by layer
      (if (or (== _index 0) (== _index_2 _returnvalue_3))
        (bind _x (.x _returnvalue_6))
        (bind _y (.y _returnvalue_6))
        (`BlueprintMapLibrary.Map_Add` (`self.LayerZValueMap`) _output_get (- _y 0.0))
        ;[1 1 1] Stores each tile bound coordinates
        (bind _output_get_2 (set `self.TileBounds` (make `/Game/IsometricTiles/TileMaps/TileCoordBounds` (+ _y _returnvalue_2) (- _y _returnvalue_2) (+ _x _returnvalue) (- _x _returnvalue))))
        (`BlueprintMapLibrary.Map_Add` (`self.TileCoordsAndBounds`) _output_get_2 (`KismetMathLibrary.MakeVector2D` _returnvalue_4 _returnvalue_5))
        ;[1 1 1] Get max and min depth of tile map.
        (bind _values (`BlueprintMapLibrary.Map_Values` _layerzvaluemap))
        (set `self.MinMaxZOfTilemapForDepth` (`KismetMathLibrary.MakeVector2D` (`|GetArrayItem` _values) (`|GetArrayItem` _values (- (`BlueprintMapLibrary.Map_Length` _layerzvaluemap) 1))))))))

(fn `GetNameValue`
  (params (ValueName :type Name))
  (returns (ReturnValue :type Name))
  (return "None"))

(fn `GetParticipantDisplayName`
  (params (ActiveSpeaker :type Name))
  (returns (ReturnValue :type Text))
  (return ""))

(fn `GetParticipantGender`
  (returns (ReturnValue :type "ETextGender Enum"))
  (return "Masculine"))

(fn `GetParticipantIcon`
  (params (ActiveSpeaker :type Name) (ActiveSpeakerState :type Name))
  (returns (ReturnValue :type "Texture2D Object Reference"))
  (return null))

(fn `GetParticipantName`
  (returns (ReturnValue :type Name))
  (return (`self.NPCName`)))

(fn `MakeDLGVisible`
  (bind _dlgwidget (`self.DLGWidget`))
  (`/Engine/EditorBlueprintResources/StandardMacros.IsValid` _dlgwidget
    (:`Is Valid`
      (`Widget.SetVisibility` _dlgwidget "Visible")
      (return))))

(fn `ModifyBoolValue`
  (params (ValueName :type Name) (bNewValue :type Boolean))
  (returns (ReturnValue :type Boolean))
  (return false))

(fn `ModifyFloatValue`
  (params (ValueName :type Name) (bDelta :type Boolean) (Value :type "Float (double-precision)"))
  (returns (ReturnValue :type Boolean))
  (return false))

(fn `ModifyIntValue`
  (params (ValueName :type Name) (bDelta :type Boolean) (Value :type Integer))
  (returns (ReturnValue :type Boolean))
  (return false))

(fn `ModifyNameValue`
  (params (ValueName :type Name) (NameValue :type Name))
  (returns (ReturnValue :type Boolean))
  (switch `name` ValueName
    (:`NPCNameOverride`
      (set `self.NPCNameOverride` NameValue)
      (return false))))

(fn `NPCCreateDLGWidget`
  (bind _returnvalue (`|CreateWidget` "/Game/UI/Dialogue/DLG_NPC_Widget.DLG_NPC_Widget_C"))
  (bind _output_get (set `self.DLGWidget` _returnvalue))
  (set `/Game/UI/Dialogue/DLG_NPC_Widget.NPCCharacter` self _output_get)
  (`UserWidget.AddToViewport` _output_get 1)
  (`Widget.SetVisibility` (`self.DLGWidget`) "Hidden")
  (`KismetSystemLibrary.PrintString` "NPC dlg widget created")
  (return))

(fn `OnDialogueEvent`
  (params (Context :type "DlgContext Object Reference") (EventName :type Name))
  (returns (ReturnValue :type Boolean))
  (return false))

(fn `RemoveDLGWidget`
  (bind _dlgwidget (`self.DLGWidget`))
  (`/Engine/EditorBlueprintResources/StandardMacros.IsValid` _dlgwidget
    (:`Is Valid`
      (`Widget.RemoveFromParent` _dlgwidget)
      (set `self.DLGWidget` null)
      (return))))

(fn `Set Sprite Depth Layer`
  (bind (_minmaxzoftilemapfordepth_x _minmaxzoftilemapfordepth_y) (`KismetMathLibrary.BreakVector2D` (`self.MinMaxZOfTilemapForDepth`)))
  (bind (_returnvalue_x _returnvalue_y) (`KismetMathLibrary.BreakVector` (`SceneComponent.K2_GetComponentLocation` (`self.CapsuleComponent`))))
  (bind _returnvalue (/ (`self.TileHeight`) 2.0))
  (`SceneComponent.K2_SetWorldLocation` (`self.Sprite`) (`KismetMathLibrary.MakeVector` _returnvalue_x (- _returnvalue_y (`self.SpriteOffset`)) (+ (`KismetMathLibrary.MapRangeClamped` (`KismetMathLibrary.Conv_IntToDouble` (* (`.ReturnValue` (`KismetMathLibrary.FMod` (+ _returnvalue_y 0.0) _returnvalue)) (`KismetMathLibrary.FTrunc` _returnvalue))) _minmaxzoftilemapfordepth_x _minmaxzoftilemapfordepth_y (* (* (- (`self.NumCosmeticLayers`) 2) (`self.LayerSeparation`)) -1.0)) 0.0)) false false)
  (return))

(fn `SetDLGTextAndName`
  (params (inNPCText :type Text) (inNPCName :type Name))
  (bind _dlgwidget (`self.DLGWidget`))
  (bind _npcname (`/Game/UI/Dialogue/DLG_NPC_Widget.NPCName` _dlgwidget))
  (`/Engine/EditorBlueprintResources/StandardMacros.IsValid` _dlgwidget
    (:`Is Valid`
      (`TextBlock.SetText` (`/Game/UI/Dialogue/DLG_NPC_Widget.NPCText` _dlgwidget) inNPCText)
      (if (`self.TriggerNameOverride`)
        (`TextBlock.SetText` _npcname (`KismetTextLibrary.Conv_NameToText` (`self.NPCNameOverride`)))
        (else
          (`TextBlock.SetText` _npcname (`KismetTextLibrary.Conv_NameToText` inNPCName))))
      (set `self.TriggerNameOverride` false)
      (return))))

(fn `SetFlipBookOnSprite`
  (bind _rightleftvaluetopass (`self.RightLeftValueToPass`))
  (bind _lastmovedirection (`self.LastMoveDirection`))
  (bind _returnvalue (> _rightleftvaluetopass 0.0))
  (bind _returnvalue_2 (< _rightleftvaluetopass 0.0))
  (bind _returnvalue_3 (== _rightleftvaluetopass 0.0))
  (bind _returnvalue_4 (* (`self.UpDownValueToPass`) -1.0))
  (bind _returnvalue_5 (< _returnvalue_4 0.0))
  (bind _returnvalue_6 (> _returnvalue_4 0.0))
  (if (or (!= (`self.UpDownValueToPass`) 0.0) (!= (`self.RightLeftValueToPass`) 0.0))
    (set `self.LastMoveDirection` (select `bool` (and _returnvalue_6 _returnvalue) :`false` (select `bool` (and _returnvalue_6 _returnvalue_3) :`false` (select `bool` (and _returnvalue_6 _returnvalue_2) :`false` (select `bool` (and (== _returnvalue_4 0.0) _returnvalue_2) :`false` (select `bool` (and _returnvalue_5 _returnvalue_2) :`false` (select `bool` (and _returnvalue_5 _returnvalue_3) :`false` (select `bool` (and _returnvalue_5 _returnvalue) :`false` "NewEnumerator1" :`true` "NewEnumerator2" :!type "/Game/Characters/EMoveDirection Enum") :`true` "NewEnumerator3") :`true` "NewEnumerator4") :`true` "NewEnumerator5") :`true` "NewEnumerator6") :`true` "NewEnumerator7") :`true` "NewEnumerator0")))
  (`PaperFlipbookComponent.SetFlipbook` (`self.Sprite`) (select `bool` (> (`KismetMathLibrary.VSize` (`self.GetVelocity`)) 0.0) :`false` (select `/Game/Characters/EMoveDirection` _lastmovedirection :`NewEnumerator0` "/Game/Characters/FlipBooks/MainCharacter/Idle_N.Idle_N" :`NewEnumerator1` "/Game/Characters/FlipBooks/MainCharacter/Idle_NE.Idle_NE" :`NewEnumerator2` "/Game/Characters/FlipBooks/MainCharacter/Idle_E.Idle_E" :`NewEnumerator3` "/Game/Characters/FlipBooks/MainCharacter/Idle_SE.Idle_SE" :`NewEnumerator4` "/Game/Characters/FlipBooks/MainCharacter/Idle_S.Idle_S" :`NewEnumerator5` "/Game/Characters/FlipBooks/MainCharacter/Idle_SW.Idle_SW" :`NewEnumerator6` "/Game/Characters/FlipBooks/MainCharacter/Idle_W.Idle_W" :`NewEnumerator7` "/Game/Characters/FlipBooks/MainCharacter/Idle_NW.Idle_NW" :!type "PaperFlipbook Object Reference") :`true` (select `/Game/Characters/EMoveDirection` _lastmovedirection :`NewEnumerator0` "/Game/Characters/FlipBooks/MainCharacter/Run_N.Run_N" :`NewEnumerator1` "/Game/Characters/FlipBooks/MainCharacter/Run_NE.Run_NE" :`NewEnumerator2` "/Game/Characters/FlipBooks/MainCharacter/Run_E.Run_E" :`NewEnumerator3` "/Game/Characters/FlipBooks/MainCharacter/Run_SE.Run_SE" :`NewEnumerator4` "/Game/Characters/FlipBooks/MainCharacter/Run_S.Run_S" :`NewEnumerator5` "/Game/Characters/FlipBooks/MainCharacter/Run_SW.Run_SW" :`NewEnumerator6` "/Game/Characters/FlipBooks/MainCharacter/Run_W.Run_W" :`NewEnumerator7` "/Game/Characters/FlipBooks/MainCharacter/Run_NW.Run_NW" :!type "PaperFlipbook Object Reference")))
  (`SceneComponent.K2_SetWorldRotation` (`self.CapsuleComponent`) (select `/Game/Characters/EMoveDirection` (`self.LastMoveDirection`) :`NewEnumerator0` (struct :`Yaw` 335.0) :`NewEnumerator2` (struct :`Yaw` 30.0) :`NewEnumerator3` (struct :`Yaw` 90.0) :`NewEnumerator4` (struct :`Yaw` 150.0) :`NewEnumerator5` (struct :`Yaw` 180.0) :`NewEnumerator6` (struct :`Yaw` 210.0) :`NewEnumerator7` (struct :`Yaw` 270.0) :!type "Rotator Structure") false false))

(fn `UserConstructionScript`
  (`SceneComponent.K2_SetWorldLocation` (`self.Sprite`) (`SceneComponent.K2_GetComponentLocation` (`self.CapsuleComponent`)) false false))