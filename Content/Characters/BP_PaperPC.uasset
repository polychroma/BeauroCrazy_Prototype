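; Player character Blueprint that drives branching conversations with BP_PaperNPC characters, plus object interaction and a computer monitor UI.
; Each Tick a forward line trace and overlap check set the dialogue state, and a value-change macro starts or ends the conversation.
; Dialogue contexts gather participants by name, show lines on NPC widgets with voice audio, and list replies selected by mouse wheel and click.
; Older overlap and interaction logic remains disconnected.
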(event `self.ReceiveBeginPlay`
  (bind _engagedindialogue (`self.EngagedInDialogue`))
  (`parent.ReceiveBeginPlay`)
  (bind _returnvalue (`|CreateWidget` "/Game/UI/WBP_BaseUI.WBP_BaseUI_C"))
  (bind _output_get (set `self.BaseUI` _returnvalue))
  (`UserWidget.AddToViewport` _output_get 0)
  (`self.AlertValueChangeTracker` _engagedindialogue _engagedindialogue))

(event `self.ReceiveTick`
  (params (DeltaSeconds :type "Float (single-precision)"))
  (`parent.ReceiveTick` DeltaSeconds)
  ;[1 1 1] Logic for Dialogue
  (`self.Line Trace to Find Actor`)
  (if (`self.EngagedInDialogue`)
    (if (or (and (!= (`self.TargettedActor`) (`self.NPC`)) (== (`self.TargettedActorClass`) "/Game/Characters/BP_PaperNPC.BP_PaperNPC_C") (`KismetArrayLibrary.Array_Contains` (`self.OverlappedCharacters`) (`self.TargettedActor`))) (not (`KismetArrayLibrary.Array_Contains` (`self.OverlappedCharacters`) (`self.NPC`))))
      (set `self.EngagedInDialogue` false)
      (bind (_oldvalue _newvalue) (`self.AlertValueChangeTracker` false (`self.EngagedInDialogue`) :!via `CheckChange` :!label _label)
        (:`ValueChanged`
          (if _newvalue
            (bind _asbp_paper_npc (cast `/Game/Characters/BP_PaperNPC` (`self.TargettedActor`)))
            (set `self.NPC` _asbp_paper_npc)
            (if (not (`/Game/Characters/BP_PaperNPC.DialogueWithNPC` _asbp_paper_npc))
              (`self.PCInitDLG`))
            (else
              (`self.EndDLGAndResetVars`))))))
    (elif (== (`self.TargettedActorClass`) "/Game/Characters/BP_PaperNPC.BP_PaperNPC_C")
      (set `self.TargetNPCInRange` (`KismetArrayLibrary.Array_Contains` (`self.OverlappedCharacters`) (`self.TargettedActor`)))
      (set `self.TargetNPCClassCheck` true)
      (bind _asbp_paper_npc_2 (cast `/Game/Characters/BP_PaperNPC` (`self.TargettedActor`)))
      (if (not (and (`KismetSystemLibrary.IsValid` (`/Game/Characters/BP_PaperNPC.DLGSelect` _asbp_paper_npc_2)) (`/Game/Characters/BP_PaperNPC.DialogueWithNPC` _asbp_paper_npc_2)))
        (set `self.EngagedInDialogue` (and (`self.TargetNPCInRange`) (`self.TargetNPCClassCheck`)))
        (goto _label :!via `CheckChange`))
      (else
        (set `self.TargetNPCClassCheck` false)))))

(event `self.DialogueRadius.OnComponentBeginOverlap`
  (params (OverlappedComponent :type "PrimitiveComponent Object Reference") (OtherActor :type "Actor Object Reference") (OtherComp :type "PrimitiveComponent Object Reference") (OtherBodyIndex :type Integer) (bFromSweep :type Boolean) (SweepResult :type "HitResult Structure (by ref)"))
  ;[1 1 1] DLG radius overlap
)

(event `self.DialogueRadius.OnComponentEndOverlap`
  (params (OverlappedComponent :type "PrimitiveComponent Object Reference") (OtherActor :type "Actor Object Reference") (OtherComp :type "PrimitiveComponent Object Reference") (OtherBodyIndex :type Integer))
  ;[1 1 1] DLG radius overlap
  ;;[1 1 1] Put this in parent so NPC can get it too.
)

(event `DialogueDown`
  (bind _dlgwidgetpc (`self.DLGWidgetPC`))
  ;[1 1 1] Dialogue Option select
  (`/Engine/EditorBlueprintResources/StandardMacros.IsValid` _dlgwidgetpc
    (:`Is Valid`
      (set `self.SelectedOption` (`KismetMathLibrary.Clamp` (+ (`self.SelectedOption`) 1) 0 (- (`PanelWidget.GetChildrenCount` (`/Game/UI/Dialogue/DLG_PC_Widget.PlayerVBox` _dlgwidgetpc)) 1)))
      (`self.HighlightSelectedReply` :!label _label_2))))

(event `DialogueUp`
  (bind _dlgwidgetpc (`self.DLGWidgetPC`))
  ;[1 1 1] Dialogue Option select
  (`/Engine/EditorBlueprintResources/StandardMacros.IsValid` _dlgwidgetpc
    (:`Is Valid`
      (set `self.SelectedOption` (`KismetMathLibrary.Clamp` (- (`self.SelectedOption`) 1) 0 (- (`PanelWidget.GetChildrenCount` (`/Game/UI/Dialogue/DLG_PC_Widget.PlayerVBox` _dlgwidgetpc)) 1)))
      (goto _label_2))))

(event `Key|MouseScrollDown`
  (params (Key :type "Key Structure"))
  (:`Pressed`
    (`/Engine/EditorBlueprintResources/StandardMacros.IsValid` (`self.DLGWidgetPC`)
      (:`Is Valid`
        (`self.DialogueDown`)))))

(event `Key|MouseScrollUp`
  (params (Key :type "Key Structure"))
  (:`Pressed`
    (`/Engine/EditorBlueprintResources/StandardMacros.IsValid` (`self.DLGWidgetPC`)
      (:`Is Valid`
        (`self.DialogueUp`)))))

(event `Key|LeftMouseButton`
  (params (Key :type "Key Structure"))
  (:`Pressed`
    (`/Engine/EditorBlueprintResources/StandardMacros.IsValid` (`self.DLGWidgetPC`)
      (:`Is Valid`
        (`self.ChooseOption`)))))

(event `InputAction|CompOpen`
  (params (Key :type "Key Structure"))
  (bind _returnvalue (`GameplayStatics.GetPlayerController` 0))
  (:`Pressed`
    (bind _returnvalue_2 (`|CreateWidget` "/Game/Computer/WBP_CompMonitor.WBP_CompMonitor_C" null null))
    (`UserWidget.AddToViewport` _returnvalue_2 0)
    (`WidgetBlueprintLibrary.SetInputMode_UIOnlyEx` _returnvalue _returnvalue_2)
    (set `PlayerController.bShowMouseCursor` true _returnvalue)))

(event `InputAction|InteractWithObject`
  (params (Key :type "Key Structure"))
  (:`Pressed`
    (`self.InteractWithObject`)))

(fn `CheckLastEdge`
  (bind _output_get (set `self.SelectedOption` 0))
  (if (`DlgContext.IsEdgeConnectedToEndNode` (`self.DLGContext`) _output_get true)
    (`DlgContext.ChooseChild` (`self.DLGContext`) (`self.SelectedOption`))
    (set `/Game/Characters/BP_PaperNPC.DLGVis` false (`self.NPC`))
    (`Widget.RemoveFromParent` (`self.DLGWidgetPC`))
    (set `self.DLGWidgetPC` null)
    (set `self.DLGDialogueSelected` null))
  (return))

(fn `ChooseOption`
  (bind _npc (`self.NPC`))
  (bind _dlgcontext (`self.DLGContext`))
  (bind _npc_2 (`self.NPC`))
  (bind _npc_3 (`self.NPC`))
  (bind _dlgwidget (`/Game/Characters/BP_PaperNPC.DLGWidget` _npc_2))
  (`/Engine/EditorBlueprintResources/StandardMacros.IsValid` (`self.DLGContext`)
    (:`Is Valid`
      (`/Engine/EditorBlueprintResources/StandardMacros.IsValid` _npc_3
        (:`Is Valid`
          (set `/Game/Characters/BP_PaperNPC.DLGVis` false _npc_3)
          (`DlgContext.ChooseChild` (`self.DLGContext`) (`self.SelectedOption`))
          (for _array_element (`self.ParticipantNPCs`)
            (if (== (`/Game/Characters/BP_PaperNPC.NPCName` _array_element) (`DlgContext.GetActiveNodeParticipantName` (`self.DLGContext`)))
              (set `self.NPC` _array_element)))
          (set `/Game/Characters/BP_PaperNPC.DLGVis` true _npc)
          (`GameplayStatics.PlaySoundAtLocation` (`DlgContext.GetActiveNodeVoiceSoundWave` (`self.DLGContext`)) (`self.K2_GetActorLocation` _npc) (struct) 1.0 1.0 0.0 null null null)
          (`/Game/Characters/BP_PaperNPC.SetDLGTextAndName` _npc_2 (`DlgContext.GetActiveNodeText` _dlgcontext) (`DlgContext.GetActiveNodeParticipantName` _dlgcontext))
          (`/Engine/EditorBlueprintResources/StandardMacros.IsValid` _dlgwidget
            (:`Is Valid`
              (`Widget.SetVisibility` _dlgwidget "Visible")
              (set `/Game/Characters/BP_PaperNPC.DialogueTimer` (`KismetSystemLibrary.GetGameTimeInSeconds`) (`self.NPC`))
              (`self.PCDLGLoop`)
              (`self.CheckLastEdge`))))
        (:`Is Not Valid`
          _)))
    (:`Is Not Valid`
      _))
  (return))

(fn `EndDLGAndResetVars`
  (bind _dlgwidgetpc (`self.DLGWidgetPC`))
  (`/Engine/EditorBlueprintResources/StandardMacros.IsValid` _dlgwidgetpc
    (:`Is Valid`
      (set `self.DLGDialogueSelected` null)
      (`Widget.RemoveFromParent` _dlgwidgetpc)
      (set `self.DLGWidgetPC` null)
      (set `self.DLGContext` null)
      (for _array_element (`self.ParticipantNPCs`)
        (set `/Game/Characters/BP_PaperNPC.DLGVis` false _array_element)
        (set `/Game/Characters/BP_PaperNPC.DialogueWithPlayer` false _array_element))
      (set `self.NPC` null)
      (`KismetArrayLibrary.Array_Clear` (`self.ParticipantNPCs`))
      (return))))

(fn `HighlightSelectedReply`
  (bind _playervbox (`/Game/UI/Dialogue/DLG_PC_Widget.PlayerVBox` (`self.DLGWidgetPC`)))
  (for _index (range (`PanelWidget.GetChildrenCount` (`/Game/UI/Dialogue/DLG_PC_Widget.PlayerVBox` (`self.DLGWidgetPC`))))
    (bind _asdlg_pc_widget_replies (cast `/Game/UI/Dialogue/DLG_PC_Widget_Replies` (`PanelWidget.GetChildAt` _playervbox _index)))
    (set `/Game/UI/Dialogue/DLG_PC_Widget_Replies.isSelected` false _asdlg_pc_widget_replies))
  (bind _asdlg_pc_widget_replies_2 (cast `/Game/UI/Dialogue/DLG_PC_Widget_Replies` (`PanelWidget.GetChildAt` _playervbox (`self.SelectedOption`))))
  (set `/Game/UI/Dialogue/DLG_PC_Widget_Replies.isSelected` true _asdlg_pc_widget_replies_2)
  (return))

(fn `Line Trace to Find Actor`
  (bind _capsulecomponent (`self.CapsuleComponent`))
  (bind _returnvalue (`SceneComponent.K2_GetComponentLocation` _capsulecomponent))
  (set `self.LastTargettedActor` (`self.TargettedActor`))
  (bind _outhit (`KismetSystemLibrary.LineTraceSingleForObjects` _returnvalue (+ _returnvalue (* (`SceneComponent.GetForwardVector` _capsulecomponent) 100.0)) (`|MakeArray` "ObjectTypeQuery7" :!type "EObjectTypeQuery Enum")))
  (bind _output_get (set `self.TargettedActor` (`.HitActor` (`GameplayStatics.BreakHitResult` _outhit))))
  (set `self.TargettedActorClass` (`GameplayStatics.GetObjectClass` _output_get))
  (return))

(fn `PCCreateDLGWidget`
  (bind _returnvalue (`|CreateWidget` "/Game/UI/Dialogue/DLG_PC_Widget.DLG_PC_Widget_C"))
  (bind _output_get (set `self.DLGWidgetPC` _returnvalue))
  (`UserWidget.AddToViewport` _output_get 0)
  (`Widget.SetVisibility` _output_get "Hidden")
  (return))

(fn `PCDLGLoop`
  (bind _dlgwidgetpc (`self.DLGWidgetPC`))
  (bind _dlgwidgetpc_2 (`self.DLGWidgetPC`))
  (`/Engine/EditorBlueprintResources/StandardMacros.IsValid` _dlgwidgetpc_2
    (:`Is Valid`
      (`PanelWidget.ClearChildren` (`/Game/UI/Dialogue/DLG_PC_Widget.PlayerVBox` _dlgwidgetpc_2))
      (set `self.SelectedOption` 0)
      (bind _output_get (set `self.NumberOfSatisfiedOptions` (- (`DlgContext.GetOptionNum` (`self.DLGContext`)) 1)))
      (for _index (range (+ _output_get 1))
        (bind _returnvalue (`|CreateWidget` "/Game/UI/Dialogue/DLG_PC_Widget_Replies.DLG_PC_Widget_Replies_C" null _dlgwidgetpc (`DlgContext.GetOptionText` (`self.DLGContext`) _index)))
        (`VerticalBox.AddChildToVerticalBox` (`/Game/UI/Dialogue/DLG_PC_Widget.PlayerVBox` _dlgwidgetpc) _returnvalue))
      (`Widget.SetVisibility` (`self.DLGWidgetPC`) "Visible")
      (`self.HighlightSelectedReply`))
    (:`Is Not Valid`
      _))
  (return))

(fn `PCInitDLG`
  (bind _dlgselect (`/Game/Characters/BP_PaperNPC.DLGSelect` (`self.NPC`)))
  (`/Engine/EditorBlueprintResources/StandardMacros.IsValid` _dlgselect
    (:`Is Valid`
      (bind _output_get (set `self.DLGDialogueSelected` _dlgselect))
      (`KismetArrayLibrary.Array_Clear` (`self.ParticipantNPCs`))
      (bind _outset (`DlgDialogue.GetAllParticipantNames` _output_get))
      (`BlueprintSetLibrary.Set_Clear` _outset)
      (bind _result (`BlueprintSetLibrary.Set_ToArray` _outset))
      (bind _output_get_2 (set `self.ParticipantNames` _result))
      (bind _outactors (`GameplayStatics.GetAllActorsOfClass` "/Game/Characters/BP_PaperNPC.BP_PaperNPC_C"))
      (for _array_element _output_get_2
        (for _array_element_2 _outactors
          (if (== (`/Game/Characters/BP_PaperNPC.NPCName` _array_element_2) _array_element)
            (set `/Game/Characters/BP_PaperNPC.DialogueWithPlayer` true _array_element_2)
            (`KismetArrayLibrary.Array_AddUnique` (`self.ParticipantNPCs`) _array_element_2))))
      (bind _returnvalue (`DlgManager.StartDialogue` (`self.DLGDialogueSelected`) (`self.ParticipantNPCs`)))
      (set `self.DLGContext` _returnvalue)
      (for _array_element_3 (`self.ParticipantNPCs`)
        (`/Engine/EditorBlueprintResources/StandardMacros.IsValid` (`/Game/Characters/BP_PaperNPC.DLGWidget` _array_element_3)
          (:`Is Not Valid`
            (`/Game/Characters/BP_PaperNPC.NPCCreateDLGWidget` _array_element_3))))
      (`/Engine/EditorBlueprintResources/StandardMacros.IsValid` (`self.DLGWidgetPC`)
        (:`Is Valid`
          _)
        (:`Is Not Valid`
          (`self.PCCreateDLGWidget`)))
      (`self.PCDLGLoop`))
    (:`Is Not Valid`
      _))
  (return))

(fn `UserConstructionScript`)