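; Player controller that manages the UINav main menu and lets the player swap control between two pawns.
; MenuOpen and CloseMenu show or remove the menu, switching input mode, cursor and pause outside the main menu level, while separate InitialMainMenu events open and close it without pausing.
; The H key flip-flops possession between the paper PC and hacker pawn; the I key sets and prints a low debug resolution in windowed fullscreen.
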(event `self.ReceiveTick`
  (params (DeltaSeconds :type "Float (single-precision)")))

(event `InputAction|MenuOpen`
  (params (Key :type "Key Structure"))
  (:`Pressed`
    (`/Engine/EditorBlueprintResources/StandardMacros.IsValid` (`self.CurrentMenu`)
      (:`Is Not Valid`
        (if (not (`self.InMainMenuLevel`))
          (bind _returnvalue (`|CreateWidget` "/Game/UI/Examples/BP_UINavMainMenu.BP_UINavMainMenu_C" self null))
          (bind _output_get (set `self.CurrentMenu` _returnvalue))
          (`UserWidget.AddToViewport` _output_get 0)
          (set `self.bShowMouseCursor` true)
          (`WidgetBlueprintLibrary.SetInputMode_UIOnlyEx` self null)
          (`GameplayStatics.SetGamePaused` true))))))

(event `CloseMenu`
  (`/Engine/EditorBlueprintResources/StandardMacros.IsValid` (`self.CurrentMenu`)
    (:`Is Valid`
      (if (not (`self.InMainMenuLevel`))
        (`Widget.RemoveFromParent` (`self.CurrentMenu`))
        (set `self.CurrentMenu` null)
        (set `self.bShowMouseCursor` false)
        (`WidgetBlueprintLibrary.SetInputMode_GameOnly` self)
        (`GameplayStatics.SetGamePaused` false)))))

(event `Key|H`
  (params (Key :type "Key Structure"))
  (:`Pressed`
    (`/Engine/EditorBlueprintResources/StandardMacros.FlipFlop`
      (:`A`
        (bind _outactors (`GameplayStatics.GetAllActorsOfClass` "/Game/Characters/BP_PaperPC.BP_PaperPC_C"))
        (`self.Possess` (`|GetArrayItem` _outactors)))
      (:`B`
        (bind _outactors_2 (`GameplayStatics.GetAllActorsOfClass` "/Game/HackMiniGame/BP_HackerPawn.BP_HackerPawn_C"))
        (`self.Possess` (`|GetArrayItem` _outactors_2))))))

(event `InitialMainMenuOpen`
  ;[1 1 1] puit something
  (bind _returnvalue (`|CreateWidget` "/Game/UI/Examples/BP_UINavMainMenu.BP_UINavMainMenu_C" self null))
  (bind _output_get (set `self.CurrentMenu` _returnvalue))
  (`UserWidget.AddToViewport` _output_get 0)
  (set `self.bShowMouseCursor` true)
  (`WidgetBlueprintLibrary.SetInputMode_UIOnlyEx` self null))

(event `Key|I`
  (params (Key :type "Key Structure"))
  (:`Pressed`
    (bind _returnvalue (`GameUserSettings.GetGameUserSettings`))
    (`GameUserSettings.SetScreenResolution` _returnvalue (make `IntPoint` 640 360))
    (bind (_returnvalue_x _returnvalue_y) (break `IntPoint` (`GameUserSettings.GetScreenResolution` _returnvalue)))
    (`KismetSystemLibrary.PrintString` (`KismetStringLibrary.Conv_IntToString` _returnvalue_x) true true (struct :`R` 1.0 :`G` 0.036018 :`A` 1.0))
    (`KismetSystemLibrary.PrintString` (`KismetStringLibrary.Conv_IntToString` _returnvalue_y) true true (struct :`G` 1.0 :`B` 0.114498 :`A` 1.0))
    (`GameUserSettings.SetFullscreenMode` _returnvalue "WindowedFullscreen")))

(event `InitialMainMenuClose`
  (`Widget.RemoveFromParent` (`self.CurrentMenu`))
  (set `self.CurrentMenu` null)
  (set `self.bShowMouseCursor` false)
  (`WidgetBlueprintLibrary.SetInputMode_GameOnly` self))

(fn `UserConstructionScript`)