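; BP_FloorTileCollision is a floor tile actor that lines up its RenderComponent with the height of the first BP_PaperPC found in the level.
; The construction script sets the component's world Z to that character's capsule Z, keeping X and Y.
; BeginPlay repeats the height match and also shifts the component back along Y by YOffset.
; Overlap and Tick events are empty.
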(event `self.ReceiveBeginPlay`
  (bind _rendercomponent (`self.RenderComponent`))
  (bind _outactors (`GameplayStatics.GetAllActorsOfClass` "/Game/Characters/BP_PaperPC.BP_PaperPC_C"))
  (`SceneComponent.K2_SetWorldLocation` _rendercomponent (`KismetMathLibrary.MakeVector` (.x (`SceneComponent.K2_GetComponentLocation` _rendercomponent)) (- (.y (`SceneComponent.K2_GetComponentLocation` _rendercomponent)) (`self.YOffset`)) (.z (`SceneComponent.K2_GetComponentLocation` (`Character.CapsuleComponent` (`|GetArrayItem` _outactors))))) false false))

(fn `UserConstructionScript`
  (bind _rendercomponent (`self.RenderComponent`))
  (bind _outactors (`GameplayStatics.GetAllActorsOfClass` "/Game/Characters/BP_PaperPC.BP_PaperPC_C"))
  (`SceneComponent.K2_SetWorldLocation` _rendercomponent (`KismetMathLibrary.MakeVector` (.x (`SceneComponent.K2_GetComponentLocation` _rendercomponent)) (.y (`SceneComponent.K2_GetComponentLocation` _rendercomponent)) (.z (`SceneComponent.K2_GetComponentLocation` (`Character.CapsuleComponent` (`|GetArrayItem` _outactors))))) false false))