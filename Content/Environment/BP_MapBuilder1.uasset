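; Map builder actor that precomputes isometric tile coordinates and depth-layer data at construction.
; The construction script maps each X/Y coordinate to a diamond-grid location from tile size, then derives ceiling and floor layer values.
; SetLayerVariables assigns descending Z values per layer and stores Y bounds for Y-to-Z depth sorting, noted as converted at runtime by PC and NPC actors.
; Its final per-tile loop is empty, with tile-center lookup disconnected.
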(fn `SetLayerVariables`
  (bind _mapsizex (`self.MapSizeX`))
  (bind _mapsizey (`self.MapSizeY`))
  (bind (_returnvalue_x _returnvalue_y) (`KismetMathLibrary.BreakVector` (`SceneComponent.K2_GetComponentLocation` (`self.DefaultSceneRoot`))))
  (bind _returnvalue (/ (`self.TileHeight`) 2.0))
  (bind _returnvalue_2 (+ _mapsizex _mapsizey))
  (bind _returnvalue_3 (- _returnvalue_y _returnvalue))
  ;[1 1 1] Get layer Z values
  (for _index (range (+ (- _returnvalue_2 2) 1))
    (if (== _index 0)
      (bind _output_get (set `self.CurrLayerZValueLoop` 0))
      (`BlueprintMapLibrary.Map_Add` (`self.LayerZValueMap`) _index _output_get)
      (else
        (bind _output_get_2 (set `self.CurrLayerZValueLoop` (- (`self.CurrLayerZValueLoop`) (`KismetMathLibrary.FTrunc` (`self.LayerSeparation`)))))
        (`BlueprintMapLibrary.Map_Add` (`self.LayerZValueMap`) _index _output_get_2))))
  (set `self.NumLayers` (`BlueprintMapLibrary.Map_Length` (`self.LayerZValueMap`)))
  ;[1 1 1] Get relevent min and max Y values to conver to Z values. real time conversion done in PC and NPC actors
  (set `self.MinMaxYForConversionToZ` (`KismetMathLibrary.MakeVector2D` _returnvalue_3 (+ _returnvalue_3 (* (- _returnvalue_2 1) _returnvalue))))
  ;[1 1 1] Loop for each X by Y in the tile map
  (for _index_2 (range _mapsizex)
    (for _index_3 (range _mapsizey)
      _)))

(fn `UserConstructionScript`
  (bind (_coordlociterator_x _coordlociterator_y) (`KismetMathLibrary.BreakVector` (`self.CoordLocIterator`)))
  (bind (_maxxycoords_x _maxxycoords_y) (`KismetMathLibrary.BreakVector2D` (`self.MaxXYCoords`)))
  (bind (_coordlociterator_x_2 _coordlociterator_y_2) (`KismetMathLibrary.BreakVector` (`self.CoordLocIterator`)))
  (bind (_returnvalue_x _returnvalue_y _returnvalue_z) (`KismetMathLibrary.BreakVector` (`SceneComponent.K2_GetComponentLocation` (`self.DefaultSceneRoot`))))
  (`BlueprintMapLibrary.Map_Clear` (`self.CoordLocMap`))
  ;[1 1 1] For X coord, set a starting point where y=0
  (for _index (range (`self.MapSizeX`))
    (set `self.CoordLocIterator` (`KismetMathLibrary.MakeVector` (* _index (* (`self.TileWidth`) 0.5)) (* _index (* (`self.TileHeight`) 0.5))))
    ;[1 1 1] for X=x, loop and increment Y, create and assign a location for coordinate
    (for _index_2 (range (`self.MapSizeY`))
      (bind _returnvalue (`KismetMathLibrary.Conv_IntToDouble` _index))
      (bind _returnvalue_2 (`KismetMathLibrary.Conv_IntToDouble` _index_2))
      (set `self.MaxXYCoords` (`KismetMathLibrary.MakeVector2D` _returnvalue _returnvalue_2))
      (`BlueprintMapLibrary.Map_Add` (`self.CoordLocMap`) (`KismetMathLibrary.MakeVector2D` _returnvalue _returnvalue_2) (`KismetMathLibrary.MakeVector` _coordlociterator_x _coordlociterator_y))
      (set `self.CoordLocIterator` (`KismetMathLibrary.MakeVector` (- _coordlociterator_x_2 (* (`self.TileWidth`) 0.5)) (+ _coordlociterator_y_2 (* (`self.TileHeight`) 0.5))))
      (`/Engine/EditorBlueprintResources/StandardMacros.IncrementInt` (`self.CoordIDCounter`))))
  (set `self.CeilingLayerValue` (* (+ (+ _maxxycoords_x _maxxycoords_y) 3.0) (`self.LayerSeparation`)))
  (set `self.FloorLayerValue` (+ _returnvalue_z (`self.FloorLayerValue`)))
  (`self.SetLayerVariables`))