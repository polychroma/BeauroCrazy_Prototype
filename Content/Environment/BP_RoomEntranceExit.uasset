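; A room trigger actor that fades a set of sprites as the BP_PaperPC player enters and leaves a room.
; Shortly after BeginPlay, it aligns the entrance and exit boxes to the player capsule's height.
; Capsule overlaps toggle InRoom: entry overrides non-special sprites' logic and sets their target opacity to InRoomOpacity, while exit restores full opacity and releases the override.
; Special-layer sprites get no change on entry.
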(event `self.ReceiveBeginPlay`
  (bind _exitbox (`self.ExitBox`))
  (bind _entrancebox (`self.EntranceBox`))
  (`KismetSystemLibrary.Delay` 1.0)
  (bind _outactors (`GameplayStatics.GetAllActorsOfClass` "/Game/Characters/BP_PaperPC.BP_PaperPC_C"))
  (bind _z (.z (`SceneComponent.K2_GetComponentLocation` (`Character.CapsuleComponent` (`|GetArrayItem` _outactors)))))
  (`SceneComponent.K2_SetWorldLocation` _entrancebox (`KismetMathLibrary.MakeVector` (.x (`SceneComponent.K2_GetComponentLocation` _entrancebox)) (.y (`SceneComponent.K2_GetComponentLocation` _entrancebox)) _z) false false)
  (`SceneComponent.K2_SetWorldLocation` _exitbox (`KismetMathLibrary.MakeVector` (.x (`SceneComponent.K2_GetComponentLocation` _exitbox)) (.y (`SceneComponent.K2_GetComponentLocation` _exitbox)) _z) false false))

(event `self.EntranceBox.OnComponentBeginOverlap`
  (params (OverlappedComponent :type "PrimitiveComponent Object Reference") (OtherActor :type "Actor Object Reference") (OtherComp :type "PrimitiveComponent Object Reference") (OtherBodyIndex :type Integer) (bFromSweep :type Boolean) (SweepResult :type "HitResult Structure (by ref)"))
  (bind _spritestocontrol (`self.SpritesToControl`))
  (if (== (`GameplayStatics.GetObjectClass` OtherActor) "/Game/Characters/BP_PaperPC.BP_PaperPC_C")
    (bind _asbp_paper_pc (cast `/Game/Characters/BP_PaperPC` OtherActor))
    (if (and (== (`Character.CapsuleComponent` _asbp_paper_pc) OtherComp) (not (`self.InRoom`)))
      (set `self.PC` _asbp_paper_pc)
      (set `self.InRoom` true)
      (if (> (`KismetArrayLibrary.Array_Length` _spritestocontrol) 0)
        (for _array_element _spritestocontrol
          (if (`/Game/Environment/BP_SpriteComponentActor.SpecialLayer` _array_element)
            (switch `/Game/Environment/ESpecialLayer` "NewEnumerator0")
            (else
              (set `/Game/Environment/BP_SpriteComponentActor.LogicOverwrittenByEntranceExit` true _array_element)
              (set `/Game/Environment/BP_SpriteComponentActor.TarOpacity` (`self.InRoomOpacity`) _array_element))))))))

(event `self.ExitBox.OnComponentBeginOverlap`
  (params (OverlappedComponent :type "PrimitiveComponent Object Reference") (OtherActor :type "Actor Object Reference") (OtherComp :type "PrimitiveComponent Object Reference") (OtherBodyIndex :type Integer) (bFromSweep :type Boolean) (SweepResult :type "HitResult Structure (by ref)"))
  (bind _spritestocontrol (`self.SpritesToControl`))
  (if (== (`GameplayStatics.GetObjectClass` OtherActor) "/Game/Characters/BP_PaperPC.BP_PaperPC_C")
    (bind _asbp_paper_pc (cast `/Game/Characters/BP_PaperPC` OtherActor))
    (if (and (== (`Character.CapsuleComponent` _asbp_paper_pc) OtherComp) (`self.InRoom`))
      (set `self.InRoom` false)
      (set `self.PC` null)
      (if (> (`KismetArrayLibrary.Array_Length` _spritestocontrol) 0)
        (for _array_element _spritestocontrol
          (set `/Game/Environment/BP_SpriteComponentActor.TarOpacity` 1.0 _array_element)
          (set `/Game/Environment/BP_SpriteComponentActor.LogicOverwrittenByEntranceExit` false _array_element)
          (`KismetSystemLibrary.PrintString` "exit"))))))

(fn `UserConstructionScript`)