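; BP_Sprite is an environment actor that displays a configurable Paper2D sprite at a height set by its tilemap layer.
; The construction script keeps the sprite's world X and Y and derives Z from the negated product of layer and separation, plus a pixel nudge.
; It then applies the default sprite; the event graph holds only disabled stub events, so nothing runs at play time.
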(fn `UserConstructionScript`
  (bind _papersprite (`self.PaperSprite`))
  (bind (_returnvalue_x _returnvalue_y) (`KismetMathLibrary.BreakVector` (`SceneComponent.K2_GetComponentLocation` _papersprite)))
  (`SceneComponent.K2_SetWorldLocation` _papersprite (`KismetMathLibrary.MakeVector` _returnvalue_x _returnvalue_y (+ (* (* (`self.TilemapLayer`) (`self.LayerSeparation`)) -1.0) (`self.PixelNudge`))) false false)
  (`PaperSpriteComponent.SetSprite` (`self.PaperSprite`) (`self.DefaultSprite`)))