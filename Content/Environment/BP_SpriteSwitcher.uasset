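; Trigger volume that hands overlapping characters and chairs its referenced Tilemap and swaps a linked sprite.
; On entry, actors refresh their sprite layer information from that map; for the player, its ceiling layer turns transparent and a differing previous map's turns opaque.
; An array tracks occupants; once empty, a Tick countdown restores the default sprite.
; BeginPlay prints a warning if Tilemap is unset.
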(event `self.ReceiveBeginPlay`
  ;[1 1 1] alert designer if actor is missing reference
  (`/Engine/EditorBlueprintResources/StandardMacros.IsValid` (`self.Tilemap`)
    (:`Is Not Valid`
      (`KismetSystemLibrary.PrintString` (`KismetStringLibrary.Concat_StrStr` (`KismetSystemLibrary.GetDisplayName` self) " does not have tilempa reference")))))

(event `self.ReceiveTick`
  (params (DeltaSeconds :type "Float (single-precision)"))
  (bind _sprite (`self.Sprite`))
  ;[1 1 1] SwitchSpriteBackToDefaultAfterTimerExpires
  (if (not (`self.bSpriteSwitchActive`))
    (bind _output_get (set `self.SwitchTimer` (- (`self.SwitchTimer`) DeltaSeconds)))
    (if (not (> _output_get 0.0))
      (`PaperSpriteComponent.SetSprite` (`/Game/Environment/BP_Sprite.PaperSprite` _sprite) (`/Game/Environment/BP_Sprite.DefaultSprite` _sprite)))))

(event `self.Trigger.OnComponentBeginOverlap`
  (params (OverlappedComponent :type "PrimitiveComponent Object Reference") (OtherActor :type "Actor Object Reference") (OtherComp :type "PrimitiveComponent Object Reference") (OtherBodyIndex :type Integer) (bFromSweep :type Boolean) (SweepResult :type "HitResult Structure (by ref)"))
  (bind _asbp_paper_character_parent (cast `/Game/Characters/BP_PaperCharacterParent` OtherActor :!pure true))
  (bind _asbp_chair_only (cast `/Game/Prototypes/Blueprints/BP_ChairOnly` OtherActor :!pure true))
  (bind _sprite (`self.Sprite`))
  (bind _tilemap (`self.Tilemap`))
  (bind _tilemap_2 (`self.Tilemap`))
  (`self.CheckActorAndCompCharacter` OtherActor OtherComp
    (:`outChar`
      ;[1 1 1] if actor is PC, then set "ceiling" layer of previous tilemap to opaque, but only if previous not equal to referenced tilemap
      (if (and (== (`GameplayStatics.GetObjectClass` OtherActor) "/Game/Characters/BP_PaperPC.BP_PaperPC_C") (!= (`/Game/Characters/BP_PaperCharacterParent.CurTilemap` _asbp_paper_character_parent) (`self.Tilemap`)))
        (`PaperTileMapComponent.SetLayerColor` (`PaperTileMapActor.RenderComponent` (`/Game/Characters/BP_PaperCharacterParent.CurTilemap` _asbp_paper_character_parent)) (struct :`R` 1.0 :`G` 1.0 :`B` 1.0 :`A` 1.0) 0))
      ;[1 1 1] set tilemap on character to the one referenced by this actor
      (set `/Game/Characters/BP_PaperCharacterParent.CurTilemap` _tilemap_2 _asbp_paper_character_parent)
      (`/Game/Characters/BP_PaperCharacterParent.GetLayerInformationForCharSprites` _asbp_paper_character_parent (`PaperTileMapActor.RenderComponent` _tilemap_2))
      ;[1 1 1] if PC, set "ceiling" layer to transparent
      (if (== (`GameplayStatics.GetObjectClass` OtherActor) "/Game/Characters/BP_PaperPC.BP_PaperPC_C")
        (`PaperTileMapComponent.SetLayerColor` :`self` (`PaperTileMapActor.RenderComponent` (`self.Tilemap`)))))
    (:`OutChair`
      ;[1 1 1] if chair, do the chair things
      (set `/Game/Prototypes/Blueprints/BP_ChairOnly.CurTilemap` _tilemap _asbp_chair_only)
      (`/Game/Prototypes/Blueprints/BP_ChairOnly.GetLayerInformationForChairSprites` _asbp_chair_only (`PaperTileMapActor.RenderComponent` _tilemap))))
  (`/Engine/EditorBlueprintResources/StandardMacros.IsValid` (`self.Sprite`)
    (:`Is Valid`
      ;[1 1 1] Set sprite in target to the switched version
      (set `self.bSpriteSwitchActive` true)
      (`PaperSpriteComponent.SetSprite` (`/Game/Environment/BP_Sprite.PaperSprite` _sprite) (`/Game/Environment/BP_Sprite.SwitchSprite` _sprite)))
    (:`Is Not Valid`
      _))
  (if true
    ;[1 1 1] keep track of how many valid actors are in the trigger volume
    (`KismetArrayLibrary.Array_AddUnique` (`self.ActorsInColBox`) OtherActor)))

(event `self.Trigger.OnComponentEndOverlap`
  (params (OverlappedComponent :type "PrimitiveComponent Object Reference") (OtherActor :type "Actor Object Reference") (OtherComp :type "PrimitiveComponent Object Reference") (OtherBodyIndex :type Integer))
  (bind _actorsincolbox (`self.ActorsInColBox`))
  (bind _sprite (`self.Sprite`))
  ;[1 1 1] if chair or char, set sprites and remove from array
  (`self.CheckActorAndCompCharacter` OtherActor OtherComp
    (:`outChar`
      _)
    (:`OutChair`
      _))
  (if (`KismetSystemLibrary.IsValid` (`self.Sprite`))
    (set `self.bSpriteSwitchActive` true)
    (`PaperSpriteComponent.SetSprite` (`/Game/Environment/BP_Sprite.PaperSprite` _sprite) (`/Game/Environment/BP_Sprite.SwitchSprite` _sprite)))
  ;[1 1 1] remove valid actor from array
  (if (`KismetArrayLibrary.Array_Contains` _actorsincolbox OtherActor)
    (`KismetArrayLibrary.Array_RemoveItem` _actorsincolbox OtherActor)
    ;[1 1 1] if no more valid actors in volume, "deactive". Sprite will switch back to default after delay. see tick
    (if (== (`KismetArrayLibrary.Array_Length` (`self.ActorsInColBox`)) 0)
      (set `self.SwitchTimer` (`self.SwitchTimerDefault`))
      (set `self.bSpriteSwitchActive` false))))

(fn `UserConstructionScript`)