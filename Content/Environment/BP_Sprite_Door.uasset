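; Sprite door for a layered Paper2D tile map that fades when the player is not in front of it.
; The construction script positions the actor from its XY coordinate via the MapBuilder's location map and layer separation, offsets the foreground and door sprites in Z, and aligns floor collision to the player capsule's height.
; Tick compares player and foreground Z, then interpolates both sprites' alpha, leaving the target untouched when LogicOverwrittenByEntranceExit is set.
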(event `self.ReceiveTick`
  (params (DeltaSeconds :type "Float (single-precision)"))
  (bind _fg (`self.FG`))
  (bind (_returnvalue_x _returnvalue_y _returnvalue_z) (`KismetMathLibrary.BreakVector` (`SceneComponent.K2_GetComponentLocation` (`self.FG`))))
  (bind (_spritecolor_r _spritecolor_g _spritecolor_b _spritecolor_a) (break `LinearColor` (`PaperSpriteComponent.SpriteColor` _fg)))
  (bind (_returnvalue_x_2 _returnvalue_y_2 _returnvalue_z_2) (`KismetMathLibrary.BreakVector` (`SceneComponent.K2_GetComponentLocation` (`PaperCharacter.Sprite` (`self.PC`)))))
  (`parent.ReceiveTick` DeltaSeconds)
  (if (not (`self.LogicOverwrittenByEntranceExit`))
    (`/Engine/EditorBlueprintResources/StandardMacros.IsValid` (`self.PC`)
      (:`Is Valid`
        (if (> _returnvalue_z_2 _returnvalue_z)
          (set `self.TarOpacity` 1.0 :!label _label)
          (else
            (set `self.TarOpacity` (`self.FadeSpriteAlpha`)))))
      (:`Is Not Valid`
        (goto _label))))
  (`PaperSpriteComponent.SetSpriteColor` _fg (make `LinearColor` _spritecolor_r _spritecolor_g _spritecolor_b (`KismetMathLibrary.FInterpTo` _spritecolor_a (`self.TarOpacity`) (`GameplayStatics.GetWorldDeltaSeconds`) 5.0)))
  (`PaperSpriteComponent.SetSpriteColor` (`self.Door`) (make `LinearColor` _spritecolor_r _spritecolor_g _spritecolor_b (`KismetMathLibrary.FInterpTo` _spritecolor_a (`self.TarOpacity`) (`GameplayStatics.GetWorldDeltaSeconds`) 5.0))))

(event `self.FloorTileCollision.OnComponentBeginOverlap`
  (params (OverlappedComponent :type "PrimitiveComponent Object Reference") (OtherActor :type "Actor Object Reference") (OtherComp :type "PrimitiveComponent Object Reference") (OtherBodyIndex :type Integer) (bFromSweep :type Boolean) (SweepResult :type "HitResult Structure (by ref)")))

(fn `UserConstructionScript`
  (bind _floortilecollision (`self.FloorTileCollision`))
  (bind (_xy_x _xy_y) (`KismetMathLibrary.BreakVector2D` (`self.XY`)))
  (bind _mapbuilderref (`self.MapBuilderRef`))
  (bind (_returnvalue_x _returnvalue_y _returnvalue_z) (`KismetMathLibrary.BreakVector` (`SceneComponent.K2_GetComponentLocation` (`self.RenderComponent`))))
  (bind (_value _returnvalue) (`BlueprintMapLibrary.Map_Find` (`/Game/Environment/BP_MapBuilder1.CoordLocMap` (`self.MapBuilderRef`)) (`KismetMathLibrary.MakeVector2D` _xy_x _xy_y)))
  (bind _returnvalue_2 (`SceneComponent.K2_GetComponentLocation` (`/Game/Environment/BP_MapBuilder1.DefaultSceneRoot` _mapbuilderref)))
  (bind _returnvalue_3 (+ _returnvalue_z (`self.DoorFGOffsetZ`)))
  (`/Engine/EditorBlueprintResources/StandardMacros.IsValid` (`self.MapBuilderRef`)
    (:`Is Valid`
      ;[1 1 1] for each sprite which has a coordinate, set a location (including Z layer). This mimics the tile map functionality. While it is less user friendly to design a map, it allows developers to access sprites directly and makes changes, for instance, to opacity. Suggested workflow is to create a tilemap and then use this actor to copy over the design.
      (set `self.LayerToSetSpriteAt` (+ (* (+ _xy_x _xy_y) (`/Game/Environment/BP_MapBuilder1.LayerSeparation` _mapbuilderref)) (.z _returnvalue_2)))
      (if _returnvalue
        (`self.K2_SetActorLocation` (`KismetMathLibrary.MakeVector` (.x _value) (- (.y _value) (`self.TileHeightOffset`)) (`self.LayerToSetSpriteAt`)))
        (bind _outactors (`GameplayStatics.GetAllActorsOfClass` "/Game/Characters/BP_PaperPC.BP_PaperPC_C"))
        (`SceneComponent.K2_SetWorldLocation` _floortilecollision (`KismetMathLibrary.MakeVector` (.x (`SceneComponent.K2_GetComponentLocation` _floortilecollision)) (.y (`SceneComponent.K2_GetComponentLocation` _floortilecollision)) (.z (`SceneComponent.K2_GetComponentLocation` (`Character.CapsuleComponent` (`|GetArrayItem` _outactors))))) false false)
        (`SceneComponent.K2_SetWorldLocation` (`self.FG`) (`KismetMathLibrary.MakeVector` _returnvalue_x _returnvalue_y _returnvalue_3) false false)
        (`SceneComponent.K2_SetWorldLocation` (`self.Door`) (`KismetMathLibrary.MakeVector` _returnvalue_x _returnvalue_y (- _returnvalue_3 0.1)) false false)
        (else
          (`self.K2_SetActorLocation` _returnvalue_2))))))