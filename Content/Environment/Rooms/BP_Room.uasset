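; Room actor that tracks which paper characters are inside it and fades assigned sprites while the player occupies it.
; Mesh overlaps set characters' current room via DetectTile, defaulting to HallWay on exit.
; The player capsule's overlaps override sprite target opacities, handling ceiling layers separately, then restore them.
; It passes lock and key settings to its door at construction and BeginPlay, and aligns its height to the player on start.
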(event `self.ReceiveBeginPlay`
  (bind _associateddoor (`self.AssociatedDoor`))
  (bind _scene (`self.Scene`))
  (bind _outactors (`GameplayStatics.GetAllActorsOfClass` "/Game/Characters/BP_PaperPC.BP_PaperPC_C"))
  (`SceneComponent.K2_SetWorldLocation` _scene (`KismetMathLibrary.MakeVector` (.x (`SceneComponent.K2_GetComponentLocation` _scene)) (.y (`SceneComponent.K2_GetComponentLocation` _scene)) (.z (`SceneComponent.K2_GetComponentLocation` (`Character.CapsuleComponent` (`|GetArrayItem` _outactors))))) false false)
  (`/Engine/EditorBlueprintResources/StandardMacros.IsValid` (`self.AssociatedTargetPoint`)
    (:`Is Valid`
      _)
    (:`Is Not Valid`
      (`KismetSystemLibrary.PrintString` (`VictoryBPFunctionLibrary.AppendMultiple` (`KismetSystemLibrary.GetDisplayName` self) " is missing a Target Point") true true (struct :`G` 0.66 :`B` 1.0 :`A` 1.0) 20.0)))
  (`/Engine/EditorBlueprintResources/StandardMacros.IsValid` _associateddoor
    (:`Is Valid`
      (set `/Game/Environment/BP_Sprite_Door.DoorLocked` (`self.RoomLocked?`) _associateddoor)
      (set `/Game/Environment/BP_Sprite_Door.KeyID` (`self.AssociatedKey`) _associateddoor)
      (set `/Game/Environment/BP_Sprite_Door.ParentRoom` self _associateddoor))))

(event `self.ReceiveTick`
  (params (DeltaSeconds :type "Float (single-precision)")))

(event `self.Tile3dStaticMesh.OnComponentBeginOverlap`
  (params (OverlappedComponent :type "PrimitiveComponent Object Reference") (OtherActor :type "Actor Object Reference") (OtherComp :type "PrimitiveComponent Object Reference") (OtherBodyIndex :type Integer) (bFromSweep :type Boolean) (SweepResult :type "HitResult Structure (by ref)"))
  (bind _spritestonotfade (`self.SpritesToNotFade`))
  (bind _spritestofade (`self.SpritesToFade`))
  (if (`KismetMathLibrary.ClassIsChildOf` (`GameplayStatics.GetObjectClass` OtherActor) "/Game/Characters/BP_PaperCharacterParent.BP_PaperCharacterParent_C")
    (bind _asbp_paper_character_parent (cast `/Game/Characters/BP_PaperCharacterParent` OtherActor))
    (if (== (`/Game/Characters/BP_PaperCharacterParent.DetectTile` _asbp_paper_character_parent) OtherComp)
      (set `/Game/Characters/BP_PaperCharacterParent.CurrentRoom` self _asbp_paper_character_parent)
      (set `/Game/Characters/BP_PaperCharacterParent.CurrentRoomName` (`self.RoomName`) _asbp_paper_character_parent))
    (if (== (`GameplayStatics.GetObjectClass` OtherActor) "/Game/Characters/BP_PaperPC.BP_PaperPC_C")
      (bind _asbp_paper_pc (cast `/Game/Characters/BP_PaperPC` OtherActor))
      (if (and (== (`Character.CapsuleComponent` _asbp_paper_pc) OtherComp) (not (`self.PlayerInRoom`)))
        (set `self.PC` _asbp_paper_pc)
        (set `self.PlayerInRoom` true)
        (if (> (`KismetArrayLibrary.Array_Length` _spritestofade) 0)
          (for _array_element _spritestofade
            (if (`/Game/Environment/BP_SpriteComponentActor.SpecialLayer` _array_element)
              (switch `/Game/Environment/ESpecialLayer` "NewEnumerator0"
                (:`NewEnumerator0`
                  (set `/Game/Environment/BP_SpriteComponentActor.LogicOverwrittenByEntranceExit` true _array_element)
                  (set `/Game/Environment/BP_SpriteComponentActor.TarOpacity` (`self.CeilingOpacity`) _array_element)))
              (else
                (set `/Game/Environment/BP_SpriteComponentActor.LogicOverwrittenByEntranceExit` true _array_element)
                (set `/Game/Environment/BP_SpriteComponentActor.TarOpacity` (`self.InRoomFadeOpacity`) _array_element)))))
        (if (> (`KismetArrayLibrary.Array_Length` _spritestonotfade) 0)
          (for _array_element_2 _spritestonotfade
            (set `/Game/Environment/BP_SpriteComponentActor.LogicOverwrittenByEntranceExit` true _array_element_2)
            (set `/Game/Environment/BP_SpriteComponentActor.TarOpacity` (`self.InRoomSolidOpacity`) _array_element_2)))))))

(event `self.Tile3dStaticMesh.OnComponentEndOverlap`
  (params (OverlappedComponent :type "PrimitiveComponent Object Reference") (OtherActor :type "Actor Object Reference") (OtherComp :type "PrimitiveComponent Object Reference") (OtherBodyIndex :type Integer))
  (bind _spritestonotfade (`self.SpritesToNotFade`))
  (bind _spritestofade (`self.SpritesToFade`))
  (if (`KismetMathLibrary.ClassIsChildOf` (`GameplayStatics.GetObjectClass` OtherActor) "/Game/Characters/BP_PaperCharacterParent.BP_PaperCharacterParent_C")
    (bind _asbp_paper_character_parent (cast `/Game/Characters/BP_PaperCharacterParent` OtherActor))
    (if (== (`/Game/Characters/BP_PaperCharacterParent.DetectTile` _asbp_paper_character_parent) OtherComp)
      (set `/Game/Characters/BP_PaperCharacterParent.CurrentRoom` null _asbp_paper_character_parent)
      (set `/Game/Characters/BP_PaperCharacterParent.CurrentRoomName` "HallWay" _asbp_paper_character_parent))
    (if (== (`GameplayStatics.GetObjectClass` OtherActor) "/Game/Characters/BP_PaperPC.BP_PaperPC_C")
      (bind _asbp_paper_pc (cast `/Game/Characters/BP_PaperPC` OtherActor))
      (if (and (== (`Character.CapsuleComponent` _asbp_paper_pc) OtherComp) (`self.PlayerInRoom`))
        (set `self.PlayerInRoom` false)
        (set `self.PC` null)
        (if (> (`KismetArrayLibrary.Array_Length` _spritestofade) 0)
          (for _array_element _spritestofade
            (set `/Game/Environment/BP_SpriteComponentActor.TarOpacity` 1.0 _array_element)
            (set `/Game/Environment/BP_SpriteComponentActor.LogicOverwrittenByEntranceExit` false _array_element)))
        (if (> (`KismetArrayLibrary.Array_Length` _spritestonotfade) 0)
          (for _array_element_2 _spritestonotfade
            (set `/Game/Environment/BP_SpriteComponentActor.TarOpacity` 1.0 _array_element_2)
            (set `/Game/Environment/BP_SpriteComponentActor.LogicOverwrittenByEntranceExit` false _array_element_2)))))))

(fn `UserConstructionScript`
  (bind _associateddoor (`self.AssociatedDoor`))
  (`/Engine/EditorBlueprintResources/StandardMacros.IsValid` _associateddoor
    (:`Is Valid`
      (set `/Game/Environment/BP_Sprite_Door.DoorLocked` (`self.RoomLocked?`) _associateddoor)
      (set `/Game/Environment/BP_Sprite_Door.KeyID` (`self.AssociatedKey`) _associateddoor)
      (set `/Game/Environment/BP_Sprite_Door.ParentRoom` self _associateddoor))
    (:`Is Not Valid`
      (`KismetSystemLibrary.PrintString` (`VictoryBPFunctionLibrary.AppendMultiple` (`KismetSystemLibrary.GetDisplayName` self) " is missing a Door") true true (struct :`G` 0.66 :`B` 1.0 :`A` 1.0) 20.0))))