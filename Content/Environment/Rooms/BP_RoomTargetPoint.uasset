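; Room target point actor that snaps its height to the BP_PaperPC character when play begins.
; On BeginPlay it finds the first BP_PaperPC and copies its capsule's world Z, keeping its own X and Y.
; The alignment happens only once; Tick and overlap events are empty, and a root-component variant of the move is left unconnected.
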(event `self.ReceiveBeginPlay`
  (bind (_returnvalue_x _returnvalue_y) (`KismetMathLibrary.BreakVector` (`self.K2_GetActorLocation` self)))
  (bind _outactors (`GameplayStatics.GetAllActorsOfClass` "/Game/Characters/BP_PaperPC.BP_PaperPC_C"))
  (`self.K2_SetActorLocation` self (`KismetMathLibrary.MakeVector` _returnvalue_x _returnvalue_y (.z (`SceneComponent.K2_GetComponentLocation` (`Character.CapsuleComponent` (`|GetArrayItem` _outactors))))) false false))

(fn `UserConstructionScript`)