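; BP_Room_Map_Helper builds lookup maps for the rooms in the level when play begins.
; It gathers every BP_Room into Rooms, then loops over them to fill two maps keyed by room.
; RoomKey stores the associated door's KeyID for rooms with a valid door and a nonzero ID.
; RoomTargetPointMap stores each room's associated target point where one is valid.
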(event `self.ReceiveBeginPlay`
  (bind _outactors (`GameplayStatics.GetAllActorsOfClass` "/Game/Environment/Rooms/BP_Room.BP_Room_C"))
  (bind _output_get (set `self.Rooms` _outactors))
  (for _array_element _output_get
    (bind _associateddoor (`/Game/Environment/Rooms/BP_Room.AssociatedDoor` _array_element))
    (bind _keyid (`/Game/Environment/BP_Sprite_Door.KeyID` _associateddoor))
    (if (and (`KismetSystemLibrary.IsValid` _associateddoor) (!= _keyid 0))
      (`BlueprintMapLibrary.Map_Add` (`self.RoomKey`) _array_element _keyid))
    (bind _associatedtargetpoint (`/Game/Environment/Rooms/BP_Room.AssociatedTargetPoint` _array_element))
    (`/Engine/EditorBlueprintResources/StandardMacros.IsValid` _associatedtargetpoint
      (:`Is Valid`
        (`BlueprintMapLibrary.Map_Add` (`self.RoomTargetPointMap`) _array_element _associatedtargetpoint)))))

(fn `UserConstructionScript`)