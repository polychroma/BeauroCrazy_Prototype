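; Hacking minigame pawn that turns gamepad stick or mouse input into an analogue direction, shown on an indicator widget and a moving sphere.
; Any key press switches input type; mouse offset from screen centre acts as a virtual stick, interpolated like real stick axes.
; A radial deadzone with per-axis sensitivity drives the sphere's offset from CenterPoint.
; Each tick while possessed, the direction becomes a normalised angle for the widget.
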(event EventBeginPlay)

(event EventTick
  (params (DeltaSeconds :type Float%20%28single-precision%29))
  (bind _centerpoint (Variables|Default|GetCenterPoint))
  (bind _returnvalue (Transformation|GetWorldLocation _centerpoint))
  (if (Variables|Refs|GetbIsPossessed)
    (CallFunction|CalcMouseAngle)
    (CallFunction|CalcAngletoSendtoWidget)
    (bind _output_get (Variables|CircleWidget|SetCircleAngle1 (Math|Float|Absolute(Float) (- (/ (Variables|CircleWidget|GetCircleAngle360) 3.6e+02) 1.0))))
    (Variables|/Game/UI/Hacking/WBP_AnalogueDirectionIndicator.WBP_AnalogueDirectionIndicator_C|SetAngleValue (Variables|CircleWidget|GetCircleWidget) _output_get)
    (Transformation|SetWorldLocation (Variables|Default|GetSphere) (Math|Vector|MakeVector (+ (.x _returnvalue) (Variables|Controls|GetLThumbX_OUT)) (+ (.y _returnvalue) (Variables|Controls|GetLThumbY_OUT)) (.z _returnvalue)) false false)))

(event EventPossessed
  (params (NewController :type Controller%20Object%20Reference))
  (bind _asbp_player_controller (Utilities|Casting|CastToBP_PlayerController NewController))
  (Variables|Refs|SetPlayerController _asbp_player_controller)
  (CallFunction|SetMouseStartParams)
  (bind _returnvalue (UserInterface|CreateWidget "/Game/UI/Hacking/WBP_AnalogueDirectionIndicator.WBP_AnalogueDirectionIndicator_C" 0 self))
  (bind _output_get (Variables|CircleWidget|SetCircleWidget _returnvalue))
  (UserInterface|Viewport|AddtoViewport _output_get 0)
  (Variables|Refs|SetbIsPossessed true)
  (Utilities|FlowControl|Delay 0.2)
  (bind _returnvalue_2 (UserInterface|CreateWidget "/Game/Debugging/WBP_Debug.WBP_Debug_C" (Game|GetPlayerController 0)))
  (UserInterface|Viewport|AddtoViewport _returnvalue_2 0))

(event EventUnpossessed
  (params (OldController :type Controller%20Object%20Reference))
  (Variables|Refs|SetbIsPossessed true))

(event Input|AxisEvents|InputAxisRightLeft
  (params (AxisValue :type Float%20%28single-precision%29))
  (switch Utilities|FlowControl|Switch|SwitchonInputType (Variables|Controls|GetInputType)
    (:NewEnumerator0
      (Variables|Controls|SetLThumbX (Math|Interpolation|FInterptoConstant (Variables|Controls|GetLThumbX) AxisValue (Utilities|Time|GetWorldDeltaSeconds) (Variables|Controls|GetControlInterpSpeed))))
    (:NewEnumerator1
      _))
  (CallFunction|RadialStickDeadzoneLogic))

(event Input|AxisEvents|InputAxisUpDown
  (params (AxisValue :type Float%20%28single-precision%29))
  (switch Utilities|FlowControl|Switch|SwitchonInputType (Variables|Controls|GetInputType)
    (:NewEnumerator0
      (Variables|Controls|SetLThumbY (Math|Interpolation|FInterptoConstant (Variables|Controls|GetLThumbY) (* AxisValue -1.0) (Utilities|Time|GetWorldDeltaSeconds) (Variables|Controls|GetControlInterpSpeed))))
    (:NewEnumerator1
      _))
  (CallFunction|RadialStickDeadzoneLogic))

(event Input|KeyboardEvents|AnyKey
  (params (Key :type Key%20Structure :default "None"))
  (bind _playercontroller (Variables|Refs|GetPlayerController))
  (:Pressed
    (if (Class|KismetInputLibrary|KeyIsGamepadKey Key)
      (bind _output_get (Variables|Controls|SetInputType "NewEnumerator0"))
      (Variables|Controls|SetInputTypeString (Utilities|String|EnumtoString _output_get))
      (Variables|/Script/Engine.PlayerController|SetbShowMouseCursor _playercontroller false)
      (elif (or (Class|KismetInputLibrary|KeyIsMouseButton Key) (Class|KismetInputLibrary|KeyIsKeyboardKey Key))
        (bind _output_get_2 (Variables|Controls|SetInputType "NewEnumerator1"))
        (Variables|Controls|SetInputTypeString (Utilities|String|EnumtoString _output_get_2))
        (Variables|/Script/Engine.PlayerController|SetbShowMouseCursor _playercontroller true)))))

(fn ConstructionScript)

(fn CalcMouseAngle
  (bind _mouselimits (Variables|Controls|GetMouseLimits))
  (bind _mouselimits_2 (Variables|Controls|GetMouseLimits))
  (switch Utilities|FlowControl|Switch|SwitchonInputType (Variables|Controls|GetInputType)
    (:NewEnumerator1
      (bind _returnvalue (Class|WidgetLayoutLibrary|GetMousePositiononViewport))
      (if (> (Math|Vector2D|Vector2DLength (- (Variables|Controls|GetMousePosStart) _returnvalue)) (Variables|Controls|GetMouseLimits))
        (Variables|Controls|SetLThumbX (Math|Interpolation|FInterptoConstant (Variables|Controls|GetLThumbX) (* (/ (.X (Math|Vector2D|BreakVector2D (* (Math|Vector2D|Normalize2D (- (Variables|Controls|GetMousePosStart) _returnvalue)) (Variables|Controls|GetMouseLimits)))) _mouselimits) -1.0) (Utilities|Time|GetWorldDeltaSeconds) (Variables|Controls|GetControlInterpSpeed)))
        (Variables|Controls|SetLThumbY (Math|Interpolation|FInterptoConstant (Variables|Controls|GetLThumbY) (* (/ (.Y (Math|Vector2D|BreakVector2D (* (Math|Vector2D|Normalize2D (- (Variables|Controls|GetMousePosStart) _returnvalue)) (Variables|Controls|GetMouseLimits)))) _mouselimits) -1.0) (Utilities|Time|GetWorldDeltaSeconds) (Variables|Controls|GetControlInterpSpeed)))
        (else
          (Variables|Controls|SetLThumbX (Math|Interpolation|FInterptoConstant (Variables|Controls|GetLThumbX) (* (/ (.X (Math|Vector2D|BreakVector2D (* (Math|Vector2D|Normalize2D (- (Variables|Controls|GetMousePosStart) _returnvalue)) (Math|Vector2D|Vector2DLength (- (Variables|Controls|GetMousePosStart) _returnvalue))))) _mouselimits_2) -1.0) (Utilities|Time|GetWorldDeltaSeconds) (Variables|Controls|GetControlInterpSpeed)))
          (Variables|Controls|SetLThumbY (Math|Interpolation|FInterptoConstant (Variables|Controls|GetLThumbY) (* (/ (.Y (Math|Vector2D|BreakVector2D (* (Math|Vector2D|Normalize2D (- (Variables|Controls|GetMousePosStart) _returnvalue)) (Math|Vector2D|Vector2DLength (- (Variables|Controls|GetMousePosStart) _returnvalue))))) _mouselimits_2) -1.0) (Utilities|Time|GetWorldDeltaSeconds) (Variables|Controls|GetControlInterpSpeed)))))
      (return))))

(fn CalcAngletoSendtoWidget
  (bind _lthumby (Variables|Controls|GetLThumbY))
  (bind _lthumbx (Variables|Controls|GetLThumbX))
  (bind _returnvalue (Class|KismetMathLibrary|DegAtan2 _lthumby _lthumbx))
  (bind _returnvalue_2 (+ _returnvalue 9e+01))
  (Variables|CircleWidget|SetATAN2Result (* _returnvalue -1.0))
  (if (< _returnvalue_2 0.0)
    (Variables|CircleWidget|SetCircleAngle360 (+ (- 9e+01 (Math|Float|Absolute(Float) _returnvalue_2)) 2.7e+02))
    (else
      (Variables|CircleWidget|SetCircleAngle360 _returnvalue_2)))
  (return))

(fn SetMouseStartParams
  (bind _returnvalue (Viewport|GetViewportSize))
  (bind _returnvalue_2 (/ _returnvalue 2.0))
  (Variables|Controls|SetMousePosStart (Math|Vector2D|MakeVector2D (.x _returnvalue_2) (.y _returnvalue_2)))
  (Class|PlayerController|SetMouseLocation (Variables|Refs|GetPlayerController) (Math|Float|Truncate (.x _returnvalue_2)) (+ (Math|Float|Truncate (.y _returnvalue_2)) 1))
  (return))

(fn RadialStickDeadzoneLogic
  (Utilities|FlowControl|Sequence
    (:then_0
      (Variables|Controls|SetMagnitude (Math|Float|Sqrt (+ (Math|Float|Power (Variables|Controls|GetLThumbX) 2.0) (Math|Float|Power (Variables|Controls|GetLThumbY) 2.0))))
      (if (> (Variables|Controls|GetMagnitude) (Variables|Controls|GetDeadzone))
        (Variables|Controls|SetAccelCurve (/ (- (Variables|Controls|GetMagnitude) (Variables|Controls|GetDeadzone)) (- (Variables|Controls|GetOuterDeadzone) (Variables|Controls|GetDeadzone))))
        (else
          (Variables|Controls|SetAccelCurve 0.0)))
      (if (> (Variables|Controls|GetAccelCurve) 1.0)
        (Variables|Controls|SetAccelCurve 1.0)))
    (:then_1
      (Variables|Controls|SetControllerAngle (Math|Trig|Atan2(Radians) (Variables|Controls|GetLThumbY) (Variables|Controls|GetLThumbX)))
      (bind _output_get (Variables|Controls|SetRefControllerAngle (Class|KismetMathLibrary|DegAtan (/ (Variables|Controls|GetLThumbY) (Variables|Controls|GetLThumbX)))))
      (Variables|Controls|SetRefControllerAngle (Math|Float|Absolute(Float) _output_get))
      (Variables|Controls|SetSensitivityScale (|(1+(({3707C750-4C48-6BE2-FC44-1595C7307319}*(({8F53164B-4A4B-BD68-F144-87902A1E3C86}/{BAAD13AA-4672-6A4F-04C0-D4A2D9A9D23F})-1))/90)))))
    (:then_2
      (Variables|Controls|SetLThumbX_OUT (|((((cos({F6A80BE9-426D-F3DA-094B-F186FBFA881A}))*{C362954C-4A16-5A9F-5789-7FA39F3BCEDB})*{BAAD13AA-4672-6A4F-04C0-D4A2D9A9D23F})*{97C93B96-4AD9-E3AC-1238-2BA5F29CDE2A}))))
    (:then_3
      (Variables|Controls|SetLThumbY_OUT (|((((sin({F6A80BE9-426D-F3DA-094B-F186FBFA881A}))*{C362954C-4A16-5A9F-5789-7FA39F3BCEDB})*{8F53164B-4A4B-BD68-F144-87902A1E3C86})*{97C93B96-4AD9-E3AC-1238-2BA5F29CDE2A})))
      (return))))