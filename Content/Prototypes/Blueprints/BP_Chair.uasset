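; BP_Chair is an interactable desk-and-chair prop that seats the character who activates it.
; On BeginPlay it stacks its layer components one unit apart along Z, descending from LayerToAnchorTo, with a slot named for the character between chair foreground and background.
; ObjectActivated extends the parent handler, disabling the character's movement, switching its capsule to overlap-only collision, flagging SittingInChair and moving it to the chair's Capsule.
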(event `self.ReceiveBeginPlay`
  (`parent.ReceiveBeginPlay`)
  (set `self.LayerIterate` (`self.LayerToAnchorTo`))
  (for _array_element (`|MakeArray` (`self.WallFG`) (`self.CompMonitor`) (`self.Hands(revisit)`) (`self.DeskAndKeys`) (`self.ChairFG`) (`self.CharLayer(LeaveBlank)`) (`self.ChairBG`) (`self.DeskBG`) (`self.WallBG`))
    (bind (_returnvalue_x _returnvalue_y) (`KismetMathLibrary.BreakVector` (`SceneComponent.K2_GetComponentLocation` _array_element)))
    (`SceneComponent.K2_SetWorldLocation` _array_element (`KismetMathLibrary.MakeVector` _returnvalue_x _returnvalue_y (`self.LayerIterate`)) false false)
    (set `self.LayerIterate` (- (`self.LayerIterate`) 1.0))))

(fn `ObjectActivated`
  (params (CharacterThatActivated :type "/Game/Characters/BP_PaperCharacterParent Object Reference"))
  (bind _capsulecomponent (`Character.CapsuleComponent` CharacterThatActivated))
  (`parent.ObjectActivated` CharacterThatActivated)
  (`CharacterMovementComponent.DisableMovement` (`Character.CharacterMovement` CharacterThatActivated))
  (`PrimitiveComponent.SetCollisionProfileName` _capsulecomponent "OverlapAllDynamic")
  (set `/Game/Characters/BP_PaperCharacterParent.SittingInChair` true CharacterThatActivated)
  (`SceneComponent.K2_SetWorldLocation` _capsulecomponent (`SceneComponent.K2_GetComponentLocation` (`self.Capsule`)) false false))

(fn `UserConstructionScript`)