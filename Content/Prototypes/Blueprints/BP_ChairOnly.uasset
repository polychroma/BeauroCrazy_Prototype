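; Interactable 2D sprite chair that seats the activating character and returns them to their prior location on deactivation.
; Activation locks movement, switches collision to overlap and snaps the occupant to the chair; deactivation reverses this, applying an eject direction.
; Tick matches foreground and background sprites to the occupant's eight-way facing.
; Depth sorting stacks both sprites along world Z from an anchor layer, with different spacing when occupied.
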(event `self.ReceiveBeginPlay`
  (`parent.ReceiveBeginPlay`)
  (`self.SetLayerOnActivation` (`|MakeArray` null null null null (`self.ChairFG`) null (`self.ChairBG`) null null null null) (`self.NotActivatedLayerIterateFloat`)))

(event `self.ReceiveTick`
  (params (DeltaSeconds :type "Float (single-precision)"))
  (`self.SetChairSprite`))

(fn `ObjectActivated`
  (params (CharacterThatActivated :type "/Game/Characters/BP_PaperCharacterParent Object Reference"))
  (bind _capsulecomponent (`Character.CapsuleComponent` CharacterThatActivated))
  (bind (_returnvalue_x _returnvalue_y _returnvalue_z) (`KismetMathLibrary.BreakVector` (`SceneComponent.K2_GetComponentLocation` (`self.Capsule`))))
  (`parent.ObjectActivated` CharacterThatActivated)
  (set `self.LocWhenInteractionHappened` (`SceneComponent.K2_GetComponentLocation` (`Character.CapsuleComponent` CharacterThatActivated)))
  (`CharacterMovementComponent.DisableMovement` (`Character.CharacterMovement` CharacterThatActivated))
  (`PrimitiveComponent.SetCollisionProfileName` _capsulecomponent "OverlapAllDynamic")
  (set `/Game/Characters/BP_PaperCharacterParent.SittingInChair` true CharacterThatActivated)
  (bind _output_get (set `self.CurChairOccupant` CharacterThatActivated))
  (set `/Game/Characters/BP_PaperCharacterParent.LastMoveDirection` (`self.LastMoveDirection`) _output_get)
  (if (`self.InFrontOfTileLayer?`)
    (`SceneComponent.K2_SetWorldLocation` _capsulecomponent (`KismetMathLibrary.MakeVector` _returnvalue_x _returnvalue_y _returnvalue_z) false false)
    (else
      (`SceneComponent.K2_SetWorldLocation` _capsulecomponent (`KismetMathLibrary.MakeVector` _returnvalue_x _returnvalue_y _returnvalue_z) false false)))
  (`self.SetLayerOnActivation` (`|MakeArray` null null null null (`self.ChairFG`) null (`self.ChairBG`) null null null null) (`self.ActivatedLayerIterateFloat`))
  (return))

(fn `ObjectDeactivated`
  (params (ActorThatDeactivated :type "/Game/Characters/BP_PaperCharacterParent Object Reference"))
  (bind _capsulecomponent (`Character.CapsuleComponent` ActorThatDeactivated))
  (`parent.ObjectDeactivated` ActorThatDeactivated)
  (bind _output_get (set `self.LastMoveDirection` (`self.ChairEjectDirection`)))
  (set `/Game/Characters/BP_PaperCharacterParent.LastMoveDirection` _output_get (`self.CurChairOccupant`))
  (`self.SetChairSprite`)
  (`SceneComponent.K2_SetWorldLocation` _capsulecomponent (`self.LocWhenInteractionHappened`) false false)
  (`CharacterMovementComponent.SetMovementMode` (`Character.CharacterMovement` ActorThatDeactivated) "MOVE_Walking" 0)
  (`PrimitiveComponent.SetCollisionProfileName` _capsulecomponent "Pawn")
  (set `/Game/Characters/BP_PaperCharacterParent.SittingInChair` false ActorThatDeactivated)
  (set `self.CurChairOccupant` null)
  (`self.SetLayerOnActivation` (`|MakeArray` null null null null (`self.ChairFG`) null (`self.ChairBG`) null null null null) (`self.NotActivatedLayerIterateFloat`))
  (return))

(fn `SetChairSprite`
  (bind _curchairoccupant (`self.CurChairOccupant`))
  (bind _lastmovedirection (`self.LastMoveDirection`))
  (`/Engine/EditorBlueprintResources/StandardMacros.IsValid` _curchairoccupant
    (:`Is Valid`
      (set `self.LastMoveDirection` (`/Game/Characters/BP_PaperCharacterParent.LastMoveDirection` _curchairoccupant))
      (`PaperSpriteComponent.SetSprite` (`self.ChairFG`) (select `/Game/Characters/EMoveDirection` _lastmovedirection :`NewEnumerator0` "/Game/SheetsSpritesSetsMaps/Sprites/OfficeObjects/deskobjects_Sprite_37.deskobjects_Sprite_37" :`NewEnumerator1` "/Game/SheetsSpritesSetsMaps/Sprites/OfficeObjects/deskobjects_Sprite_38.deskobjects_Sprite_38" :`NewEnumerator2` "/Game/SheetsSpritesSetsMaps/Sprites/OfficeObjects/deskobjects_Sprite_39.deskobjects_Sprite_39" :`NewEnumerator4` "/Game/SheetsSpritesSetsMaps/Sprites/OfficeObjects/deskobjects_Sprite_33.deskobjects_Sprite_33" :`NewEnumerator5` "/Game/SheetsSpritesSetsMaps/Sprites/OfficeObjects/deskobjects_Sprite_34.deskobjects_Sprite_34" :`NewEnumerator6` "/Game/SheetsSpritesSetsMaps/Sprites/OfficeObjects/deskobjects_Sprite_35.deskobjects_Sprite_35" :`NewEnumerator7` "/Game/SheetsSpritesSetsMaps/Sprites/OfficeObjects/deskobjects_Sprite_28.deskobjects_Sprite_28" :!type "PaperSprite Object Reference"))
      (`PaperSpriteComponent.SetSprite` (`self.ChairBG`) (select `/Game/Characters/EMoveDirection` _lastmovedirection :`NewEnumerator0` "/Game/SheetsSpritesSetsMaps/Sprites/OfficeObjects/deskobjects_Sprite_28.deskobjects_Sprite_28" :`NewEnumerator1` "/Game/SheetsSpritesSetsMaps/Sprites/OfficeObjects/deskobjects_Sprite_30.deskobjects_Sprite_30" :`NewEnumerator2` "/Game/SheetsSpritesSetsMaps/Sprites/OfficeObjects/deskobjects_Sprite_31.deskobjects_Sprite_31" :`NewEnumerator3` "/Game/SheetsSpritesSetsMaps/Sprites/OfficeObjects/deskobjects_Sprite_24.deskobjects_Sprite_24" :`NewEnumerator4` "/Game/SheetsSpritesSetsMaps/Sprites/OfficeObjects/deskobjects_Sprite_25.deskobjects_Sprite_25" :`NewEnumerator5` "/Game/SheetsSpritesSetsMaps/Sprites/OfficeObjects/deskobjects_Sprite_26.deskobjects_Sprite_26" :`NewEnumerator6` "/Game/SheetsSpritesSetsMaps/Sprites/OfficeObjects/deskobjects_Sprite_27.deskobjects_Sprite_27" :`NewEnumerator7` "/Game/SheetsSpritesSetsMaps/Sprites/OfficeObjects/deskobjects_Sprite_28.deskobjects_Sprite_28" :!type "PaperSprite Object Reference"))
      (return))))

(fn `SetLayerOnActivation`
  (params (Layers :type "Array of PaperSpriteComponent Object Reference") (LayerIterateIn :type "Float (double-precision)"))
  (if (`self.InFrontOfTileLayer?`)
    (set `self.LayerIterate` (+ (`self.LayerToAnchorTo`) (`self.SpriteSeparation`)))
    (else
      (set `self.LayerIterate` (`self.LayerToAnchorTo`))))
  (for _array_element Layers
    (`/Engine/EditorBlueprintResources/StandardMacros.IsValid` _array_element
      (:`Is Valid`
        (bind (_returnvalue_x _returnvalue_y) (`KismetMathLibrary.BreakVector` (`SceneComponent.K2_GetComponentLocation` _array_element)))
        (`SceneComponent.K2_SetWorldLocation` _array_element (`KismetMathLibrary.MakeVector` _returnvalue_x _returnvalue_y (`self.LayerIterate`)) false false))
      (:`Is Not Valid`
        _))
    (set `self.LayerIterate` (- (`self.LayerIterate`) LayerIterateIn)))
  (return))

(fn `UserConstructionScript`)