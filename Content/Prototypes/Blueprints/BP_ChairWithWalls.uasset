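; Interactable 2D office chair, with desk and wall sprites, that a character can sit in.
; BeginPlay stacks the sprite layers along Z from an anchor layer, leaving a slot for the character between chair foreground and background.
; Activation disables the character's movement, switches its capsule to overlap and moves it onto the seat.
; Tick swaps both chair sprites to match the occupant's last eight-way facing direction.
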(event `self.ReceiveBeginPlay`
  (`parent.ReceiveBeginPlay`)
  (set `self.LayerIterate` (`self.LayerToAnchorTo`))
  (for _array_element (`|MakeArray` (`self.WallFG`) (`self.CompMonitor`) (`self.Hands(revisit)`) (`self.DeskAndKeys`) (`self.ChairFG`) (`self.CharLayer(LeaveBlank)`) (`self.ChairBG`) (`self.DeskBG`) (`self.WallBG`))
    (bind (_returnvalue_x _returnvalue_y) (`KismetMathLibrary.BreakVector` (`SceneComponent.K2_GetComponentLocation` _array_element)))
    (`SceneComponent.K2_SetWorldLocation` _array_element (`KismetMathLibrary.MakeVector` _returnvalue_x _returnvalue_y (`self.LayerIterate`)) false false)
    (set `self.LayerIterate` (- (`self.LayerIterate`) 1.0))))

(event `self.ReceiveTick`
  (params (DeltaSeconds :type "Float (single-precision)"))
  (`self.SetChairSprite`))

(fn `ObjectActivated`
  (params (CharacterThatActivated :type "/Game/Characters/BP_PaperCharacterParent Object Reference"))
  (bind _capsulecomponent (`Character.CapsuleComponent` CharacterThatActivated))
  (bind (_returnvalue_x _returnvalue_y _returnvalue_z) (`KismetMathLibrary.BreakVector` (`SceneComponent.K2_GetComponentLocation` (`self.Capsule`))))
  (`parent.ObjectActivated` CharacterThatActivated)
  (`CharacterMovementComponent.DisableMovement` (`Character.CharacterMovement` CharacterThatActivated))
  (`PrimitiveComponent.SetCollisionProfileName` _capsulecomponent "OverlapAllDynamic")
  (set `/Game/Characters/BP_PaperCharacterParent.SittingInChair` true CharacterThatActivated)
  (`SceneComponent.K2_SetWorldLocation` _capsulecomponent (`KismetMathLibrary.MakeVector` _returnvalue_x (+ _returnvalue_y (`self.PlayerCapsuleOffsetWhenSeated`)) _returnvalue_z) false false)
  (set `self.CurChairOccupant` CharacterThatActivated))

(fn `SetChairSprite`
  (bind _curchairoccupant (`self.CurChairOccupant`))
  (bind _lastmovedirection (`self.LastMoveDirection`))
  (`/Engine/EditorBlueprintResources/StandardMacros.IsValid` _curchairoccupant
    (:`Is Valid`
      (set `self.LastMoveDirection` (`/Game/Characters/BP_PaperCharacterParent.LastMoveDirection` _curchairoccupant))
      (`PaperSpriteComponent.SetSprite` (`self.ChairFG`) (select `/Game/Characters/EMoveDirection` _lastmovedirection :`NewEnumerator0` "/Game/SheetsSpritesSetsMaps/Sprites/OfficeObjects/deskobjects_Sprite_37.deskobjects_Sprite_37" :`NewEnumerator1` "/Game/SheetsSpritesSetsMaps/Sprites/OfficeObjects/deskobjects_Sprite_38.deskobjects_Sprite_38" :`NewEnumerator2` "/Game/SheetsSpritesSetsMaps/Sprites/OfficeObjects/deskobjects_Sprite_39.deskobjects_Sprite_39" :`NewEnumerator4` "/Game/SheetsSpritesSetsMaps/Sprites/OfficeObjects/deskobjects_Sprite_33.deskobjects_Sprite_33" :`NewEnumerator5` "/Game/SheetsSpritesSetsMaps/Sprites/OfficeObjects/deskobjects_Sprite_34.deskobjects_Sprite_34" :`NewEnumerator6` "/Game/SheetsSpritesSetsMaps/Sprites/OfficeObjects/deskobjects_Sprite_35.deskobjects_Sprite_35" :`NewEnumerator7` "/Game/SheetsSpritesSetsMaps/Sprites/OfficeObjects/deskobjects_Sprite_28.deskobjects_Sprite_28" :!type "PaperSprite Object Reference"))
      (`PaperSpriteComponent.SetSprite` (`self.ChairBG`) (select `/Game/Characters/EMoveDirection` _lastmovedirection :`NewEnumerator0` "/Game/SheetsSpritesSetsMaps/Sprites/OfficeObjects/deskobjects_Sprite_28.deskobjects_Sprite_28" :`NewEnumerator1` "/Game/SheetsSpritesSetsMaps/Sprites/OfficeObjects/deskobjects_Sprite_30.deskobjects_Sprite_30" :`NewEnumerator2` "/Game/SheetsSpritesSetsMaps/Sprites/OfficeObjects/deskobjects_Sprite_31.deskobjects_Sprite_31" :`NewEnumerator3` "/Game/SheetsSpritesSetsMaps/Sprites/OfficeObjects/deskobjects_Sprite_24.deskobjects_Sprite_24" :`NewEnumerator4` "/Game/SheetsSpritesSetsMaps/Sprites/OfficeObjects/deskobjects_Sprite_25.deskobjects_Sprite_25" :`NewEnumerator5` "/Game/SheetsSpritesSetsMaps/Sprites/OfficeObjects/deskobjects_Sprite_26.deskobjects_Sprite_26" :`NewEnumerator6` "/Game/SheetsSpritesSetsMaps/Sprites/OfficeObjects/deskobjects_Sprite_27.deskobjects_Sprite_27" :`NewEnumerator7` "/Game/SheetsSpritesSetsMaps/Sprites/OfficeObjects/deskobjects_Sprite_28.deskobjects_Sprite_28" :!type "PaperSprite Object Reference")))))

(fn `UserConstructionScript`)