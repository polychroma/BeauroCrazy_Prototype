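; BP_SecurityCard is a prototype security card interactable that snaps to a tile on the map builder's grid.
; Construction Script and BeginPlay both look up its XY coordinate in MapBuilderRef's location map, using logic copied from BP_SpriteComponentActor.
; Z derives from X+Y layer separation plus an optional override for sprite sorting, while the interact volume gets its own Z.
; Activation calls the parent, prints a debug message and returns false.
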(event `self.ReceiveBeginPlay`
  (bind _interactvol (`self.InteractVol`))
  (bind (_xy_x _xy_y) (`KismetMathLibrary.BreakVector2D` (`self.XY`)))
  (bind _mapbuilderref (`self.MapBuilderRef`))
  (bind (_returnvalue_x _returnvalue_y) (`KismetMathLibrary.BreakVector` (`SceneComponent.K2_GetComponentLocation` _interactvol)))
  (bind (_value _returnvalue) (`BlueprintMapLibrary.Map_Find` (`/Game/Environment/BP_MapBuilder1.CoordLocMap` (`self.MapBuilderRef`)) (`KismetMathLibrary.MakeVector2D` _xy_x _xy_y)))
  (bind _returnvalue_2 (`SceneComponent.K2_GetComponentLocation` (`/Game/Environment/BP_MapBuilder1.DefaultSceneRoot` _mapbuilderref)))
  ;[1 1 1] This functionality is taken from BP_SpriteComponentActor. Allows designer to affix this actor to a tile and then customize
  (`/Engine/EditorBlueprintResources/StandardMacros.IsValid` (`self.MapBuilderRef`)
    (:`Is Valid`
      ;;[1 1 1] for each sprite which has a coordinate, set a location (including Z layer). This mimics the tile map functionality. While it is less user friendly to design a map, it allows developers to access sprites directly and makes changes, for instance, to opacity. Suggested workflow is to create a tilemap and then use this actor to copy over the design.
      (`SceneComponent.K2_SetWorldLocation` _interactvol (`KismetMathLibrary.MakeVector` _returnvalue_x _returnvalue_y (`self.ZLoc`)) false false)
      (set `self.LayerToSetSpriteAt` (+ (* (+ _xy_x _xy_y) (`/Game/Environment/BP_MapBuilder1.LayerSeparation` _mapbuilderref)) (.z _returnvalue_2)))
      (if (`self.OverrideLayer?`)
        (set `self.LayerToSetSpriteAt` (+ (`self.LayerToSetSpriteAt`) (`self.OverrideLayerOffset`))))
      (if _returnvalue
        (`self.K2_SetActorLocation` (`KismetMathLibrary.MakeVector` (+ (.x _returnvalue_2) (.x _value)) (- (+ (.y _returnvalue_2) (.y _value)) (`self.TileHeightOffset`)) (`self.LayerToSetSpriteAt`)))
        (else
          (`self.K2_SetActorLocation` _returnvalue_2))))))

(fn `ObjectActivated2`
  (params (ActorThatActivated :type "/Game/Characters/BP_PaperCharacterParent Object Reference"))
  (returns (Interaction2 :type Boolean))
  (`parent.ObjectActivated2` ActorThatActivated)
  (`KismetSystemLibrary.PrintString` "card activated")
  (return false))

(fn `UserConstructionScript`
  (bind _interactvol (`self.InteractVol`))
  (bind (_xy_x _xy_y) (`KismetMathLibrary.BreakVector2D` (`self.XY`)))
  (bind _mapbuilderref (`self.MapBuilderRef`))
  (bind (_returnvalue_x _returnvalue_y) (`KismetMathLibrary.BreakVector` (`SceneComponent.K2_GetComponentLocation` _interactvol)))
  (bind (_value _returnvalue) (`BlueprintMapLibrary.Map_Find` (`/Game/Environment/BP_MapBuilder1.CoordLocMap` (`self.MapBuilderRef`)) (`KismetMathLibrary.MakeVector2D` _xy_x _xy_y)))
  (bind _returnvalue_2 (`SceneComponent.K2_GetComponentLocation` (`/Game/Environment/BP_MapBuilder1.DefaultSceneRoot` _mapbuilderref)))
  ;[1 1 1] This functionality is taken from BP_SpriteComponentActor. Allows designer to affix this actor to a tile and then customize
  (`/Engine/EditorBlueprintResources/StandardMacros.IsValid` (`self.MapBuilderRef`)
    (:`Is Valid`
      ;;[1 1 1] for each sprite which has a coordinate, set a location (including Z layer). This mimics the tile map functionality. While it is less user friendly to design a map, it allows developers to access sprites directly and makes changes, for instance, to opacity. Suggested workflow is to create a tilemap and then use this actor to copy over the design.
      (`SceneComponent.K2_SetWorldLocation` _interactvol (`KismetMathLibrary.MakeVector` _returnvalue_x _returnvalue_y (`self.ZLoc`)) false false)
      (set `self.LayerToSetSpriteAt` (+ (* (+ _xy_x _xy_y) (`/Game/Environment/BP_MapBuilder1.LayerSeparation` _mapbuilderref)) (.z _returnvalue_2)))
      (if (`self.OverrideLayer?`)
        (set `self.LayerToSetSpriteAt` (+ (`self.LayerToSetSpriteAt`) (`self.OverrideLayerOffset`))))
      (if _returnvalue
        (`self.K2_SetActorLocation` (`KismetMathLibrary.MakeVector` (+ (.x _returnvalue_2) (.x _value)) (- (+ (.y _returnvalue_2) (.y _value)) (`self.TileHeightOffset`)) (`self.LayerToSetSpriteAt`)))
        (else
          (`self.K2_SetActorLocation` _returnvalue_2))))))