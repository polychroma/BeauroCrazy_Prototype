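; Static interactable sprite actor that places itself on a grid defined by a map builder, mimicking a tilemap while keeping each sprite directly editable.
; The construction script looks up its XY coordinate in the builder's location map and derives Z depth from coordinate sum, special ceiling/floor layers, override or foreground offsets.
; On BeginPlay, it moves its interaction volume to the Z height of the first BP_PaperPC's capsule.
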(event `self.ReceiveBeginPlay`
  (bind _interactvol (`self.InteractVol`))
  (bind (_returnvalue_x _returnvalue_y) (`KismetMathLibrary.BreakVector` (`SceneComponent.K2_GetComponentLocation` _interactvol)))
  (`parent.ReceiveBeginPlay`)
  (bind _outactors (`GameplayStatics.GetAllActorsOfClass` "/Game/Characters/BP_PaperPC.BP_PaperPC_C"))
  (bind (_returnvalue_x_2 _returnvalue_y_2 _returnvalue_z) (`KismetMathLibrary.BreakVector` (`SceneComponent.K2_GetComponentLocation` (`Character.CapsuleComponent` (`|GetArrayItem` _outactors)))))
  (`SceneComponent.K2_SetWorldLocation` _interactvol (`KismetMathLibrary.MakeVector` _returnvalue_x _returnvalue_y _returnvalue_z) false false))

(fn `UserConstructionScript`
  (bind (_xy_x _xy_y) (`KismetMathLibrary.BreakVector2D` (`self.XY`)))
  (bind _mapbuilderref (`self.MapBuilderRef`))
  (bind _mapbuilderref_2 (`self.MapBuilderRef`))
  (bind (_value _returnvalue) (`BlueprintMapLibrary.Map_Find` (`/Game/Environment/BP_MapBuilder1.CoordLocMap` (`self.MapBuilderRef`)) (`KismetMathLibrary.MakeVector2D` _xy_x _xy_y)))
  (bind _returnvalue_2 (`SceneComponent.K2_GetComponentLocation` (`/Game/Environment/BP_MapBuilder1.DefaultSceneRoot` _mapbuilderref)))
  (`parent.UserConstructionScript`)
  (`/Engine/EditorBlueprintResources/StandardMacros.IsValid` (`self.MapBuilderRef`)
    (:`Is Valid`
      ;[1 1 1] for each sprite which has a coordinate, set a location (including Z layer). This mimics the tile map functionality. While it is less user friendly to design a map, it allows developers to access sprites directly and makes changes, for instance, to opacity. Suggested workflow is to create a tilemap and then use this actor to copy over the design.
      (if (`self.SpecialLayer`)
        (switch `/Game/Environment/ESpecialLayer` (`self.SpecialLayerName`)
          (:`NewEnumerator0`
            (set `self.LayerToSetSpriteAt` (`/Game/Environment/BP_MapBuilder1.CeilingLayerValue` _mapbuilderref_2)))
          (:`NewEnumerator1`
            (set `self.LayerToSetSpriteAt` (`/Game/Environment/BP_MapBuilder1.FloorLayerValue` _mapbuilderref_2))))
        (else
          (set `self.LayerToSetSpriteAt` (+ (* (+ _xy_x _xy_y) (`/Game/Environment/BP_MapBuilder1.LayerSeparation` _mapbuilderref)) (.z _returnvalue_2)))))
      (if (`self.OverrideLayer?`)
        (set `self.LayerToSetSpriteAt` (+ (`self.LayerToSetSpriteAt`) (`self.OverrideLayerOffset`)))
        (elif (`self.Foreground`)
          (set `self.LayerToSetSpriteAt` (+ (`self.LayerToSetSpriteAt`) (`self.ForegroundZPlaneRaise`)))))
      (if _returnvalue
        (set `self.XYWorldValues` (`KismetMathLibrary.MakeVector2D` (.x _value) (.y _value)))
        (`self.K2_SetActorLocation` (`KismetMathLibrary.MakeVector` (.x _value) (- (.y _value) (`self.TileHeightOffset`)) (`self.LayerToSetSpriteAt`)))
        (else
          (`self.K2_SetActorLocation` _returnvalue_2))))))