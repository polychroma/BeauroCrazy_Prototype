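; BP_Time is an in-game clock actor that scales a configurable day length into hours and minutes and counts days.
; While TimeUpdates is on, Tick advances the time and builds a zero-padded HH:MM string.
; At midnight it increments the day, jumps to 08:00 and turns TimeUpdates off.
; A value-tracker macro watches the integer minute and calls the SendTimeUpdate dispatcher when it changes.
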(event `self.ReceiveBeginPlay`
  (bind _minuteint (`self.MinuteInt`))
  ;[1 1 1] Set Time params on BeginPlay
  (bind _output_get (set `self.OneDay` (* (`self.DayLengthInSeconds`) 1.0)))
  (set `self.OneHour` (/ _output_get 24.0))
  (set `self.Hour` 0.0)
  ;[1 1 1] Setup check for time change var
  (`self.AlertValueChangeTracker` _minuteint _minuteint))

(event `self.ReceiveTick`
  (params (DeltaSeconds :type "Float (single-precision)"))
  ;[1 1 1] Time ticking and day increment
  (`self.TickTime` DeltaSeconds)
  (`self.GenerateTimeString`)
  ;[1 1 1] If time variable changes, perhaps fire an event dispatcher?
  (`self.AlertValueChangeTracker` 0 (`self.MinuteInt`) :!via `CheckChange`
    (:`ValueChanged`
      (`self.SendTimeUpdate`))))

(fn `GenerateTimeString`
  (bind _hourint (`self.HourInt`))
  (bind _minuteint (`self.MinuteInt`))
  (bind _returnvalue (`KismetStringLibrary.Conv_IntToString` _minuteint))
  (bind _returnvalue_2 (`KismetStringLibrary.Conv_IntToString` _hourint))
  (if (> _hourint 9)
    (set `self.HourString` _returnvalue_2)
    (else
      (set `self.HourString` (`KismetStringLibrary.Concat_StrStr` "0" _returnvalue_2))))
  (if (> _minuteint 9)
    (set `self.MinString` _returnvalue)
    (else
      (set `self.MinString` (`KismetStringLibrary.Concat_StrStr` "0" _returnvalue))))
  (set `self.TimeString` (`KismetStringLibrary.Concat_StrStr` (`self.HourString`) ":" (`self.MinString`)))
  (return))

(fn `IncrementDay`
  (`/Engine/EditorBlueprintResources/StandardMacros.IncrementInt` (`self.DayCounter`)
    (:`  `
      (set `self.TimeUpdates` false)
      (set `self.Hour` 8.0)
      (return))))

(fn `TickTime`
  (params (DeltaSeconds :type "Float (double-precision)"))
  (returns (NewParam :type Boolean))
  (bind _hour (`self.Hour`))
  (bind _returnvalue (+ (`self.Hour`) (/ DeltaSeconds (`self.OneHour`))))
  (if (`self.TimeUpdates`)
    (if (>= _returnvalue 24.0)
      (set `self.Hour` 0.0)
      (`self.IncrementDay`)
      (else
        (set `self.Hour` _returnvalue)))
    (set `self.Minute` (`KismetMathLibrary.Conv_IntToDouble` (`KismetMathLibrary.FTrunc` (* (* (- _hour (`KismetMathLibrary.Conv_IntToDouble` (`KismetMathLibrary.FTrunc` _hour))) 0.6) 100.0))))
    (set `self.HourInt` (`KismetMathLibrary.FTrunc` (`self.Hour`)))
    (set `self.MinuteInt` (`KismetMathLibrary.FTrunc` (`self.Minute`)))
    (return false)))

(fn `UserConstructionScript`)